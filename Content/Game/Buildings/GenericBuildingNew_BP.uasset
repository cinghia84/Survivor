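; Searchable building that highlights under the cursor and is randomly rolled as infested at construction.
; Clicking an infested building spawns a group of zombies on the ground behind the player, clearing the infestation once one finds ground.
; Otherwise, the first click spawns random hidden items into its found list, and every click opens the paused search menu.
; A helper reports free storage space from the found items' sizes.
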(event OnBeginCursorOver(Box)
  (params (TouchedComponent :type Primitive%20Component%20Object%20Reference))
  (Rendering|SetVisibility (Variables|Default|GetHighLightCube) true false))

(event OnEndCursorOver(Box)
  (params (TouchedComponent :type Primitive%20Component%20Object%20Reference))
  (Rendering|SetVisibility (Variables|Default|GetHighLightCube) false false))

(event OnClicked(Box)
  (params (TouchedComponent :type Primitive%20Component%20Object%20Reference) (ButtonPressed :type Key%20Structure :default "AnyKey"))
  (bind _returnvalue (Game|GetPlayerController 0))
  (bind _returnvalue_2 (Pawn|GetControlledPawn _returnvalue))
  (if (not (Variables|Default|GetInfested))
    (if (Variables|Default|GetInspected)
      _
      (else
        (CallFunction|SpawnItemsin)
        (Variables|Default|SetInspected true)))
    (bind _returnvalue_3 (UserInterface|CreateWidget "/Game/Game/Menu/buildingSearchMenu.BuildingSearchMenu_C"))
    (UserInterface|Viewport|AddtoViewport _returnvalue_3 0)
    (Game|SetGamePaused true)
    (Variables|/Game/Game/Menu/buildingSearchMenu.BuildingSearchMenu_C|SetBuilding _returnvalue_3 self)
    (bind _astop_down_character (Utilities|Casting|CastToTopDownCharacter (Pawn|GetControlledPawn (Game|GetPlayerController 0))))
    (Variables|/Game/Game/Menu/buildingSearchMenu.BuildingSearchMenu_C|SetPawn _returnvalue_3 _astop_down_character)
    (Default|Init _returnvalue_3)
    (else
      (for _index (range 0 6)
        (bind (_return_value _hit) (CallFunction|HitGroundLocation (+ (Transformation|GetActorLocation _returnvalue_2) (* (Transformation|GetActorForwardVector _returnvalue_2) (Math|Random|RandomFloatinRange -2e+02 -5e+01)) (* (Transformation|GetActorRightVector _returnvalue_2) (Math|Random|RandomFloatinRange -1.5e+02 1.5e+02))) 2e+02 (Utilities|Array|MakeArray _returnvalue_2)))
        (if _hit
          (Game|SpawnActorfromClass "/Game/Characters/Zombie/Zombie_BP.Zombie_BP_C" (Math|Conversions|ToTransform(Vector) _return_value) "Undefined" 0 0)
          (Variables|Default|SetInfested false))))))

(event EventBeginPlay)

(event Collision|EventActorBeginOverlap
  (params (OtherActor :type Actor%20Object%20Reference)))

(event EventTick
  (params (DeltaSeconds :type Float%20%28single-precision%29)))

(fn ConstructionScript
  (Variables|Default|SetInfested (Math|Random|RandomBoolwithWeight 0.6)))

(fn SpawnItemsin
  (bind _itemstospawn (Variables|Default|GetItemsToSpawn))
  (bind _returnvalue (Utilities|Array|Length _itemstospawn))
  (bind (_return_value _hit _rotator) (CallFunction|HitGroundLocation (Transformation|GetActorLocation) 2.0 (Utilities|Array|MakeArray self)))
  (for _index (range 0 (Math|Random|RandomIntegerinRange 0 _returnvalue))
    (bind _returnvalue_2 (Game|SpawnActorfromClass (Utilities|Array|Get(acopy) _itemstospawn (Math|Random|RandomIntegerinRange 0 _returnvalue)) (Math|Transform|MakeTransform _return_value (Math|Rotator|MakeRotator (.Roll (Math|Rotator|BreakRotator _rotator)) 0.0 (.Yaw (Math|Rotator|BreakRotator _rotator)))) "AlwaysSpawn" 0 0))
    (Utilities|IsValid _returnvalue_2
      (:Is%20Valid
        (Rendering|SetActorHiddenInGame _returnvalue_2 true)
        (Utilities|Array|Add (Variables|Default|GetItemsFound) _returnvalue_2)))))

(fn StorageSpaceFree
  (for _array_element (Variables|Default|GetItemsFound)
    (LocalVariables|SetStorageInUse (+ (LocalVariables|GetStorageInUse) (Variables|/Game/Game/Code/ObjectGen.ObjectGen_C|GetSpace _array_element))))
  (return (- (Variables|Default|GetSpace) (LocalVariables|GetStorageInUse))))