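; Generic building actor that randomizes its rooms and cleans up overlapping walls when SetBuilding runs.
; Each room child actor component swaps to a random class from that room's RoomsTypeArray.
; A second pass over the room child actors uses overlap queries to destroy walls touching door walls and window walls touching plain walls.
; Overlapping door walls also get DestroyDoor called before removal.
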(event Custom|SetBuilding
  (for _array_element (Components|GetChildrenComponents (Variables|Default|GetDefaultSceneRoot) false)
    (bind _aschild_actor_component (Utilities|Casting|CastToChildActorComponent _array_element))
    (Utilities|Casting|CastToGenericRoom_BP (Variables|/Script/Engine.ChildActorComponent|GetChildActor _aschild_actor_component))
    (CallFunction|SetRoomsType _aschild_actor_component))
  (for _array_element_2 (Actor|GetAllChildActors false)
    (Utilities|Casting|CastToGenericRoom_BP _array_element_2)
    (CallFunction|RemoveWallandWindows _array_element_2)))

(event Collision|EventActorBeginOverlap
  (params (OtherActor :type Actor%20Object%20Reference)))

(event EventTick
  (params (DeltaSeconds :type Float%20%28single-precision%29)))

(fn ConstructionScript)

(fn RemoveWallandWindows
  (params (ChildActor :type Actor%20Object%20Reference))
  (for _array_element (Actor|GetAllChildActors ChildActor false)
    (Utilities|IsValid _array_element
      (:Is%20Valid
        (bind _aswall_door_bp (Utilities|Casting|CastToWall_Door_BP _array_element)
          (:then
            (for _array_element_2 (Collision|GetOverlappingActors _aswall_door_bp "/Game/Game/Code/Rooms/GenericWall_BP.GenericWall_BP_C" :!class /Script/Engine.Actor)
              (Utilities|IsValid _array_element_2
                (:Is%20Valid
                  (bind _aswall_door_bp_2 (Utilities|Casting|CastToWall_Door_BP _array_element_2)
                    (:then
                      (Default|DestroyDoor _aswall_door_bp_2))
                    (:CastFailed
                      _))
                  (Actor|DestroyActor _array_element_2)))))
          (:CastFailed
            (bind _aswall_bp (Utilities|Casting|CastToWall_BP _array_element))
            (for _array_element_3 (Collision|GetOverlappingActors _aswall_bp "/Game/Game/Code/Rooms/Wall_Window_BP.Wall_Window_BP_C" :!class /Script/Engine.Actor)
              (Utilities|IsValid _array_element_3
                (:Is%20Valid
                  (Actor|DestroyActor _array_element_2))))))))))

(fn SetRoomsType
  (params (ChildActor :type Child%20Actor%20Component%20Object%20Reference))
  (bind _asgeneric_room_bp (Utilities|Casting|CastToGenericRoom_BP (Variables|/Script/Engine.ChildActorComponent|GetChildActor ChildActor)))
  (if (> (Utilities|Array|Length (Variables|/Game/Game/Code/GenericRoom_BP.GenericRoom_BP_C|GetRoomsTypeArray _asgeneric_room_bp)) 0)
    (ChildActorComponent|SetChildActorClass ChildActor (Utilities|Array|Get(acopy) (Variables|/Game/Game/Code/GenericRoom_BP.GenericRoom_BP_C|GetRoomsTypeArray _asgeneric_room_bp) (Math|Random|RandomIntegerinRange 0 (Utilities|Array|LastIndex (Variables|/Game/Game/Code/GenericRoom_BP.GenericRoom_BP_C|GetRoomsTypeArray _asgeneric_room_bp)))))))