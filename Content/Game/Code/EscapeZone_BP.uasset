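; EscapeZone_BP is an escape area that ends the match when a player reaches it as the driver of a car.
; On box overlap it ignores sphere components and checks that the TopDownCharacter has a valid car and is its driver.
; It then adds bonus points to each TopDownCharacter on board that car and calls EndGame on the TopDownGameMode.
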(event OnComponentBeginOverlap(Box)
  (params (OverlappedComponent :type Primitive%20Component%20Object%20Reference) (OtherActor :type Actor%20Object%20Reference) (OtherComp :type Primitive%20Component%20Object%20Reference) (OtherBodyIndex :type Integer) (bFromSweep :type Boolean) (SweepResult :type Hit%20Result%20Structure%20%28by%20ref%29))
  (bind _astop_down_character (Utilities|Casting|CastToTopDownCharacter OtherActor))
  (if (!= (Utilities|GetClass OtherComp) "/Script/Engine.SphereComponent")
    (Utilities|IsValid (Variables|/Game/TopDownBP/Blueprints/TopDownCharacter.TopDownCharacter_C|GetCar _astop_down_character)
      (:Is%20Valid
        (if (Variables|/Game/TopDownBP/Blueprints/TopDownCharacter.TopDownCharacter_C|GetisDriver _astop_down_character)
          (for _array_element (Variables|/Game/Game/Code/GenericCar_BP.GenericCar_BP_C|GetPawnOnBoard (Variables|/Game/TopDownBP/Blueprints/TopDownCharacter.TopDownCharacter_C|GetCar _astop_down_character))
            (bind _astop_down_character_2 (Utilities|Casting|CastToTopDownCharacter _array_element))
            (Variables|/Game/TopDownBP/Blueprints/TopDownCharacter.TopDownCharacter_C|SetPoints _astop_down_character_2 (+ (Variables|/Game/TopDownBP/Blueprints/TopDownCharacter.TopDownCharacter_C|GetPoints _astop_down_character_2) 10)))
          (bind _astop_down_game_mode (Utilities|Casting|CastToTopDownGameMode (Game|GetGameMode)))
          (Default|EndGame _astop_down_game_mode))))))

(event EventBeginPlay)

(event Collision|EventActorBeginOverlap
  (params (OtherActor :type Actor%20Object%20Reference)))

(event EventTick
  (params (DeltaSeconds :type Float%20%28single-precision%29)))

(fn ConstructionScript)