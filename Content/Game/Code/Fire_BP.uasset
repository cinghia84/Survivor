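; Fire hazard actor that harms players, zombies and cars touching its collision.
; A cast chain on begin overlap takes one Health from a TopDownCharacter, ignoring its sphere components.
; Living zombies are stopped after a delay, play a death animation, and are flagged dead after another delay.
; Cars eject everyone on board through GetOut and are then destroyed.
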(event OnComponentBeginOverlap(FireCollision)
  (params (OverlappedComponent :type Primitive%20Component%20Object%20Reference) (OtherActor :type Actor%20Object%20Reference) (OtherComp :type Primitive%20Component%20Object%20Reference) (OtherBodyIndex :type Integer) (bFromSweep :type Boolean) (SweepResult :type Hit%20Result%20Structure%20%28by%20ref%29))
  ;[1 1 1] OverlapOnFire
  (bind _astop_down_character (Utilities|Casting|CastToTopDownCharacter OtherActor)
    (:then
      (if (!= (Utilities|GetClass OtherComp) "/Script/Engine.SphereComponent")
        (Math|Integer|DecrementInt (Variables|/Game/TopDownBP/Blueprints/TopDownCharacter.TopDownCharacter_C|GetHealth _astop_down_character))))
    (:CastFailed
      (bind _aszombie_bp (Utilities|Casting|CastToZombie_BP OtherActor)
        (:then
          (Utilities|IsValid _aszombie_bp
            (:Is%20Valid
              (if (not (Variables|/Game/Characters/Zombie/Zombie_BP.Zombie_BP_C|GetisDead _aszombie_bp))
                (bind _returnvalue (AI|GetAIController _aszombie_bp))
                (Utilities|FlowControl|Delay 1.0)
                (AI|Navigation|StopMovement _returnvalue)
                (Components|Animation|PlayAnimation (Variables|/Script/Engine.Character|GetMesh _aszombie_bp) "/Game/Characters/Zombie/zombie_death.zombie_death" false)
                (Utilities|FlowControl|Delay 3.0)
                (Variables|/Game/Characters/Zombie/Zombie_BP.Zombie_BP_C|SetisDead _aszombie_bp true)))))
        (:CastFailed
          (bind _asgeneric_car_bp (Utilities|Casting|CastToGenericCar_BP OtherActor))
          (Utilities|IsValid _asgeneric_car_bp
            (:Is%20Valid
              (for _array_element (Variables|/Game/Game/Code/GenericCar_BP.GenericCar_BP_C|GetPawnOnBoard _asgeneric_car_bp)
                (Default|GetOut _asgeneric_car_bp _array_element))
              (Actor|DestroyActor _asgeneric_car_bp))))))))

(event EventBeginPlay)

(fn ConstructionScript
  (|CallParentFunction))