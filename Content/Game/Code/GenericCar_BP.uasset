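; Drivable car that hides boarded pawns and follows the first one, aligning to the ground and making zombie-attracting noise while started.
; Each tick, zombies overlapping the attack capsule of the moving car trigger a roll of capacity minus zombie count plus d6: eject occupants and damage car, push zombies back, or kill for points.
; Fuel, keys and incident are randomized at BeginPlay.
; Hover highlights the car; clicking within range opens a pausing CarMenu.
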(event OnBeginCursorOver(Box)
  (params (TouchedComponent :type Primitive%20Component%20Object%20Reference))
  (bind _staticmesh (Variables|Default|GetStaticMesh))
  (bind _output_get (Variables|Default|SetMaterials (Rendering|Material|GetMaterials _staticmesh)))
  (CallFunction|HighlightObject _staticmesh _output_get "/Game/Game/Code/MaterialHighlight/M_Highlight.M_Highlight" true))

(event OnEndCursorOver(Box)
  (params (TouchedComponent :type Primitive%20Component%20Object%20Reference))
  (CallFunction|HighlightObject (Variables|Default|GetStaticMesh) (Variables|Default|GetMaterials) 0 false))

(event OnClicked(Box)
  (params (TouchedComponent :type Primitive%20Component%20Object%20Reference) (ButtonPressed :type Key%20Structure :default "AnyKey"))
  (bind _returnvalue (Game|Player|GetPlayerPawn 0))
  (Class|NavMovementComponent|StopActiveMovement (Pawn|GetMovementComponent _returnvalue))
  (bind _returnvalue_2 (CallFunction|DistanceTrace _returnvalue self "ObjectTypeQuery15"))
  (if _returnvalue_2
    (bind _returnvalue_3 (UserInterface|CreateWidget "/Game/Game/Menu/CarMenu.CarMenu_C"))
    (UserInterface|Viewport|AddtoViewport _returnvalue_3 0)
    (bind _output_get (Variables|Default|SetWidget _returnvalue_3))
    (Variables|/Game/Game/Menu/CarMenu.CarMenu_C|SetCar _output_get self)
    (Game|SetGamePaused true)))

(event Custom|GetOnBoard
  (params (Pawn :type Top%20Down%20Character%20Object%20Reference))
  (bind _self self)
  (bind _pawnonboard (Variables|Default|GetPawnOnBoard))
  (bind _returnvalue (Transformation|GetActorLocation _self))
  (bind (_x _y) (Math|Vector|BreakVector _returnvalue))
  (if (< (Utilities|Array|Length _pawnonboard) (Variables|Default|GetCapacity))
    (Transformation|SetActorRotation Pawn (Math|Rotator|MakeRotator 0.0 0.0 (.Yaw (Math|Rotator|BreakRotator (Transformation|GetActorRotation _self)))))
    (Transformation|SetActorLocation Pawn (Math|Vector|MakeVector _x _y (.Z (Math|Vector|BreakVector (Transformation|GetActorLocation Pawn)))) false false)
    (Utilities|Array|Add _pawnonboard Pawn)
    (Rendering|SetActorHiddenInGame Pawn true)
    (Variables|/Game/TopDownBP/Blueprints/TopDownCharacter.TopDownCharacter_C|SetCar Pawn self)
    (else
      (Development|PrintString "Full" true false "(R=0.000000,G=0.660000,B=1.000000,A=1.000000)" 3.0))))

(event Custom|GetOut
  (params (Pawn :type Top%20Down%20Character%20Object%20Reference))
  (Utilities|Array|RemoveItem (Variables|Default|GetPawnOnBoard) Pawn)
  (Rendering|SetActorHiddenInGame Pawn false)
  (Variables|/Game/TopDownBP/Blueprints/TopDownCharacter.TopDownCharacter_C|SetCar Pawn 0)
  (Transformation|SetActorLocation Pawn (+ (Transformation|GetActorLocation Pawn) (* (Transformation|GetActorRightVector Pawn) -3e+02)) true true)
  (Collision|SetActorEnableCollision Pawn true))

(event EventBeginPlay
  (bind _returnvalue (Math|Random|RandomBoolwithWeight 0.5))
  (Transformation|SetActorRotation "0, 0,-90.000000")
  (Variables|Default|SetFuel _returnvalue)
  (Variables|Default|SetIncident _returnvalue)
  (Variables|Default|SetKeysIn _returnvalue))

(event Collision|EventActorBeginOverlap
  (params (OtherActor :type Actor%20Object%20Reference)))

(event EventTick
  (params (DeltaSeconds :type Float%20%28single-precision%29))
  (bind _self self)
  (bind _pawnonboard (Variables|Default|GetPawnOnBoard))
  (bind _pawnonboard_2 (Variables|Default|GetPawnOnBoard))
  (bind _item (Utilities|Array|Get(acopy) _pawnonboard_2))
  (bind _returnvalue (Transformation|GetActorLocation _item))
  (bind (_x _y) (Math|Vector|BreakVector _returnvalue))
  (Utilities|FlowControl|Sequence
    (:then_0
      (if (> (Utilities|Array|Length _pawnonboard_2) 0)
        (bind (_return_value _hit _rotator) (CallFunction|HitGroundLocation _returnvalue 1e+01 _pawnonboard_2))
        (Transformation|SetActorLocation _self (Math|Vector|MakeVector _x _y (.Z (Math|Vector|BreakVector _return_value))) true false)
        (Transformation|SetActorRotation _self (Math|Rotator|MakeRotator -9e+01 (- 9e+01 (.Pitch (Math|Rotator|BreakRotator _rotator))) (.Yaw (Math|Rotator|BreakRotator (Transformation|GetActorRotation _item)))))))
    (:then_1
      (CallFunction|ZombieAttack))
    (:then_2
      (Rendering|SetVisibility (Variables|Default|GetFireDamaged) (Variables|Default|GetDamaged) true))
    (:then_3
      (if (and (> (Utilities|Array|Length _pawnonboard) 0) (Variables|Default|GetStarted))
        (CallFunction|ZombieNoiseMovement (Utilities|Array|Get(acopy) _pawnonboard))
        (CallFunction|SetTimeStartNoise)))))

(fn ConstructionScript
  (Transformation|SetActorScale3D "2.300000,1.000000,2.000000")
  (Transformation|SetWorldRotation (Variables|Default|GetFireDamaged) (Math|Rotator|MakeRotator 0.0 0.0 (Math|Random|RandomFloatinRange -1.8e+02 1.8e+02)) false false))

(fn IsonBoard
  (params (Pawn :type Top%20Down%20Character%20Object%20Reference))
  (return (>= (Utilities|Array|FindItem (Variables|Default|GetPawnOnBoard) Pawn) 0)))

(fn ZombieAttack
  (bind _returnvalue (Transformation|GetActorLocation))
  (bind _returnvalue_2 (Math|Random|RandomIntegerinRange 1 6))
  (bind _capacity (Variables|Default|GetCapacity))
  (bind _attackcapsule (Variables|Default|GetAttackCapsule))
  (bind _pawnonboard (Variables|Default|GetPawnOnBoard))
  (bind _pawnonboard_2 (Variables|Default|GetPawnOnBoard))
  (bind _item (Utilities|Array|Get(acopy) _pawnonboard_2))
  (bind _item_2 (Utilities|Array|Get(acopy) _pawnonboard))
  (bind (_x _y) (Math|Vector|BreakVector _returnvalue))
  (bind _overlappingactors (Collision|GetOverlappingActors _attackcapsule "/Game/Characters/Zombie/Zombie_BP.Zombie_BP_C" :!class /Script/Engine.PrimitiveComponent))
  (bind _returnvalue_3 (Utilities|Array|Length _overlappingactors))
  (bind _returnvalue_4 (- _capacity _returnvalue_3))
  (bind _returnvalue_5 (+ _returnvalue_4 _returnvalue_2))
  (Utilities|IsValid _item_2
    (:Is%20Valid
      (if (and (> (Utilities|Array|Length _overlappingactors) 0) (> (Math|Vector|VectorLength (Transformation|GetVelocity _item_2)) 0.0))
        (LocalVariables|SetOverlapZombieArray _overlappingactors)
        (if (<= _returnvalue_5 1)
          (for _array_element (Variables|Default|GetPawnOnBoard)
            (CallFunction|GetOut _array_element))
          (Variables|Default|SetDamaged true)
          (CallFunction|DrawTextonScreen "NewEnumerator3")
          (else
            (switch int _returnvalue_5
              (:Default
                (for _array_element_2 (LocalVariables|GetOverlapZombieArray)
                  (bind _aszombie_bp (Utilities|Casting|CastToZombie_BP _array_element_2))
                  (if (not (Variables|/Game/Characters/Zombie/Zombie_BP.Zombie_BP_C|GetisDead _aszombie_bp))
                    (Components|Animation|PlayAnimation (Variables|/Script/Engine.Character|GetMesh _aszombie_bp) "/Game/Characters/Zombie/zombie_death.zombie_death" false)
                    (Variables|/Game/Characters/Zombie/Zombie_BP.Zombie_BP_C|SetisDead _aszombie_bp true)
                    (Math|Integer|IncrementInt (Variables|/Game/TopDownBP/Blueprints/TopDownCharacter.TopDownCharacter_C|GetPoints _item)
                      (:%20%20
                        (CallFunction|DrawTextonScreen "NewEnumerator7")
                        (Audio|PlaySound2D "/Game/Game/Audio/Hit_cue.Hit_cue"))))))
              (:2
                (for _array_element_3 (LocalVariables|GetOverlapZombieArray) :!label _label
                  (bind _aszombie_bp_2 (Utilities|Casting|CastToZombie_BP _array_element_3))
                  (if (not (Variables|/Game/Characters/Zombie/Zombie_BP.Zombie_BP_C|GetisDead _aszombie_bp_2))
                    (Default|MoveBack _aszombie_bp_2 _item)
                    (Utilities|IsValid 0
                      (:Is%20Valid
                        (Transformation|SetActorLocation _aszombie_bp_2 (Math|Vector|MakeVector _x _y (.Z (Math|Vector|BreakVector (Transformation|GetActorLocation _aszombie_bp_2)))) true true))
                      (:Is%20Not%20Valid
                        _))
                    (CallFunction|DrawTextonScreen "NewEnumerator7")
                    (Audio|PlaySound2D "/Game/Game/Audio/Hit_cue.Hit_cue"))))
              (:3
                (goto _label))
              (:4
                (goto _label))
              (:5
                (goto _label)))))))))