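; Base room actor that tracks which characters and zombies occupy it through a box trigger, setting their Room and Floor.
; Tick re-applies this to overlapping characters and calls the overridable SetRoofVisibility.
; First-access Shed or Cellar entry rolls a random value, boosted when power is on, for the overridable Search event.
; SearchRoomResult shows a search menu and pauses the game; DestroyWall removes child wall and door actors.
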(event OnComponentBeginOverlap(Box)
  (params (OverlappedComponent :type Primitive%20Component%20Object%20Reference) (OtherActor :type Actor%20Object%20Reference) (OtherComp :type Primitive%20Component%20Object%20Reference) (OtherBodyIndex :type Integer) (bFromSweep :type Boolean) (SweepResult :type Hit%20Result%20Structure%20%28by%20ref%29))
  (bind _self self)
  (bind _astop_down_character (Utilities|Casting|CastToTopDownCharacter OtherActor)
    (:then
      (if (!= (Utilities|GetClass OtherComp) "/Script/Engine.SphereComponent")
        (bind _output_get (Variables|/Game/TopDownBP/Blueprints/TopDownCharacter.TopDownCharacter_C|SetRoom _astop_down_character _self))
        (Variables|/Game/TopDownBP/Blueprints/TopDownCharacter.TopDownCharacter_C|SetFloor _astop_down_character (Variables|Default|GetFloor))
        (bind _asshed_bp (Utilities|Casting|CastToShed_BP _output_get)
          (:then
            (if (Variables|/Game/Game/Images/Rooms/Blueprint/Shed_BP.Shed_BP_C|GetFirstAccess _asshed_bp)
              (CallFunction|SearchValue :!label _label)))
          (:CastFailed
            (bind _ascellar_bp (Utilities|Casting|CastToCellar_BP _output_get))
            (if (Variables|/Game/Game/Images/Rooms/Blueprint/Cellar_BP.Cellar_BP_C|GetFirstAccess _ascellar_bp)
              (goto _label))))))
    (:CastFailed
      (bind _aszombie_bp (Utilities|Casting|CastToZombie_BP OtherActor))
      (Variables|/Game/Characters/Zombie/Zombie_BP.Zombie_BP_C|SetRoom _aszombie_bp _self)
      (Variables|/Game/Characters/Zombie/Zombie_BP.Zombie_BP_C|SetFloor _aszombie_bp (Variables|Default|GetFloor)))))

(event OnComponentEndOverlap(Box)
  (params (OverlappedComponent :type Primitive%20Component%20Object%20Reference) (OtherActor :type Actor%20Object%20Reference) (OtherComp :type Primitive%20Component%20Object%20Reference) (OtherBodyIndex :type Integer))
  (bind _astop_down_character (Utilities|Casting|CastToTopDownCharacter OtherActor)
    (:then
      (if (!= (Utilities|GetClass OtherComp) "/Script/Engine.SphereComponent")
        (Variables|/Game/TopDownBP/Blueprints/TopDownCharacter.TopDownCharacter_C|SetRoom _astop_down_character 0)
        (Variables|/Game/TopDownBP/Blueprints/TopDownCharacter.TopDownCharacter_C|SetFloor _astop_down_character 0)))
    (:CastFailed
      (bind _aszombie_bp (Utilities|Casting|CastToZombie_BP OtherActor)
        (:then
          (Variables|/Game/Characters/Zombie/Zombie_BP.Zombie_BP_C|SetRoom _aszombie_bp 0)
          (Variables|/Game/Characters/Zombie/Zombie_BP.Zombie_BP_C|SetFloor _aszombie_bp 0))
        (:CastFailed
          (bind _asobject_gen (Utilities|Casting|CastToObjectGen OtherActor))
          (Variables|/Game/Game/Code/ObjectGen.ObjectGen_C|SetRoom _asobject_gen 0))))))

(event Custom|Search
  (params (Value :type Integer)))

(event Custom|SetRoofVisibility)

(event EventBeginPlay)

(event Collision|EventActorBeginOverlap
  (params (OtherActor :type Actor%20Object%20Reference)))

(event EventTick
  (params (DeltaSeconds :type Float%20%28single-precision%29))
  (Utilities|FlowControl|Sequence
    (:then_0
      (for _array_element (Collision|GetOverlappingActors (Variables|Default|GetBox) "/Game/TopDownBP/Blueprints/TopDownCharacter.TopDownCharacter_C" :!class /Script/Engine.PrimitiveComponent)
        (bind _astop_down_character (Utilities|Casting|CastToTopDownCharacter _array_element))
        (Variables|/Game/TopDownBP/Blueprints/TopDownCharacter.TopDownCharacter_C|SetRoom _astop_down_character self)
        (Variables|/Game/TopDownBP/Blueprints/TopDownCharacter.TopDownCharacter_C|SetFloor _astop_down_character (Variables|Default|GetFloor))))
    (:then_1
      (CallFunction|SetRoofVisibility))))

(fn ConstructionScript
  (Transformation|SetActorRelativeScale3D "3.000000,3.000000,3.000000"))

(fn SearchValue
  (LocalVariables|SetValue (Math|Random|RandomIntegerinRange 1 6))
  (bind _astop_down_game_mode (Utilities|Casting|CastToTopDownGameMode (Game|GetGameMode)))
  (if (Variables|/Game/TopDownBP/Blueprints/TopDownGameMode.TopDownGameMode_C|GetPowerOn _astop_down_game_mode)
    (Math|Integer|IncrementInt (LocalVariables|GetValue)
      (:%20%20
        _)))
  (Utilities|Casting|CastToTopDownCharacter (Game|Player|GetPlayerPawn 0))
  (CallFunction|Search (LocalVariables|GetValue)))

(fn SearchRoomResult
  (params (object :type Object%20Gen%20Object%20Reference))
  (bind _returnvalue (UserInterface|CreateWidget "/Game/Game/Menu/SearchMenu.SearchMenu_C"))
  (UserInterface|Viewport|AddtoViewport _returnvalue 0)
  (Default|Init _returnvalue object)
  (Game|SetGamePaused true))

(fn CheckPawn)

(fn DestroyWall
  (for _array_element (Components|GetChildrenComponents (Variables|Default|GetDefaultSceneRoot) true)
    (bind _aschild_actor_component (Utilities|Casting|CastToChildActorComponent _array_element))
    (bind _asgeneric_wall_bp (Utilities|Casting|CastToGenericWall_BP (Variables|/Script/Engine.ChildActorComponent|GetChildActor _aschild_actor_component))
      (:then
        (Actor|DestroyActor _asgeneric_wall_bp))
      (:CastFailed
        (bind _asdoor_bp (Utilities|Casting|CastToDoor_BP (Variables|/Script/Engine.ChildActorComponent|GetChildActor _aschild_actor_component)))
        (Actor|DestroyActor _asdoor_bp)))))