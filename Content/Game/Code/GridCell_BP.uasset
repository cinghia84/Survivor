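; A single grid tile that tracks who stands on it and provides cell-based checks for throwing and fire.
; Box overlap stamps X/Y onto characters and zombies, steers zombies without Noise near its center, and resets highlights when characters leave.
; Functions compare grid distance to health-scaled range, open a paused throw menu if a line trace hits only cells, and spawn fire.
; Click-to-move, highlighting and room detection logic is unwired.
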(event OnClicked(StaticMeshComponent)
  (params (TouchedComponent :type Primitive%20Component%20Object%20Reference) (ButtonPressed :type Key%20Structure :default "AnyKey")))

(event OnComponentBeginOverlap(Box)
  (params (OverlappedComponent :type Primitive%20Component%20Object%20Reference) (OtherActor :type Actor%20Object%20Reference) (OtherComp :type Primitive%20Component%20Object%20Reference) (OtherBodyIndex :type Integer) (bFromSweep :type Boolean) (SweepResult :type Hit%20Result%20Structure%20%28by%20ref%29))
  (bind _returnvalue (Math|Random|RandomFloatinRange 0.0 5e+01))
  (bind _self self)
  (bind _returnvalue_2 (Transformation|GetActorLocation _self))
  (bind (_x _y _z) (Math|Vector|BreakVector _returnvalue_2))
  (bind _astop_down_character (Utilities|Casting|CastToTopDownCharacter OtherActor)
    (:then
      (if (!= (Utilities|GetClass OtherComp) "/Script/Engine.SphereComponent")
        (Variables|/Game/TopDownBP/Blueprints/TopDownCharacter.TopDownCharacter_C|SetX _astop_down_character (Variables|Default|GetX))
        (Variables|/Game/TopDownBP/Blueprints/TopDownCharacter.TopDownCharacter_C|SetY _astop_down_character (Variables|Default|GetY))))
    (:CastFailed
      (bind _aszombie_bp (Utilities|Casting|CastToZombie_BP OtherActor))
      (Variables|/Game/Characters/Zombie/Zombie_BP.Zombie_BP_C|SetX _aszombie_bp (Variables|Default|GetX))
      (Variables|/Game/Characters/Zombie/Zombie_BP.Zombie_BP_C|SetY _aszombie_bp (Variables|Default|GetY))
      (if (not (Variables|/Game/Characters/Zombie/Zombie_BP.Zombie_BP_C|GetNoise _aszombie_bp))
        (bind _returnvalue_3 (AI|GetAIController _aszombie_bp))
        (AI|Navigation|SimpleMovetoLocation _returnvalue_3 (Math|Vector|MakeVector (+ _x _returnvalue) (+ _y _returnvalue) _z))))))

(event OnComponentEndOverlap(Box)
  (params (OverlappedComponent :type Primitive%20Component%20Object%20Reference) (OtherActor :type Actor%20Object%20Reference) (OtherComp :type Primitive%20Component%20Object%20Reference) (OtherBodyIndex :type Integer))
  (Utilities|Casting|CastToTopDownCharacter OtherActor)
  (if (!= (Utilities|GetClass OtherComp) "/Script/Engine.SphereComponent")
    (CallFunction|ResetAllCellMaterial)))

(fn ConstructionScript)

(fn CheckIsValidDistance
  (bind _astop_down_character (Utilities|Casting|CastToTopDownCharacter (Game|Player|GetPlayerPawn 0)))
  (return (<= (Math|Integer|Max(Integer) (Math|Integer|Absolute(Integer) (- (Variables|Default|GetX) (Variables|/Game/TopDownBP/Blueprints/TopDownCharacter.TopDownCharacter_C|GetX _astop_down_character))) (Math|Integer|Absolute(Integer) (- (Variables|Default|GetY) (Variables|/Game/TopDownBP/Blueprints/TopDownCharacter.TopDownCharacter_C|GetY _astop_down_character)))) (Math|Float|Truncate (* (Variables|/Game/TopDownBP/Blueprints/TopDownCharacter.TopDownCharacter_C|GetHealth _astop_down_character) (Variables|/Game/TopDownBP/Blueprints/TopDownCharacter.TopDownCharacter_C|GetMultiplier _astop_down_character))))))

(fn CheckDropObject
  (bind _astop_down_character (Utilities|Casting|CastToTopDownCharacter (Game|Player|GetPlayerPawn 0)))
  (bind _return_value (CallFunction|CalcDistanceCell self _astop_down_character))
  (Utilities|IsValid (Variables|/Game/TopDownBP/Blueprints/TopDownCharacter.TopDownCharacter_C|GetWeaponL_R _astop_down_character)
    (:Is%20Valid
      (if (>= (Math|Float|Truncate (* (Variables|/Game/TopDownBP/Blueprints/TopDownCharacter.TopDownCharacter_C|GetHealth _astop_down_character) (Variables|/Game/TopDownBP/Blueprints/TopDownCharacter.TopDownCharacter_C|GetMultiplier _astop_down_character))) _return_value) :!label _label
        (bind _canthrow (CallFunction|CheckFreeLine _astop_down_character self))
        (if _canthrow
          (bind _returnvalue (UserInterface|CreateWidget "/Game/Game/Menu/ThrowObjectMenu.ThrowObjectMenu_C"))
          (UserInterface|Viewport|AddtoViewport _returnvalue 0)
          (Variables|/Game/Game/Menu/ThrowObjectMenu.ThrowObjectMenu_C|SetCell _returnvalue self)
          (Game|SetGamePaused true))))
    (:Is%20Not%20Valid
      (if (or (Utilities|IsValid (Variables|/Game/TopDownBP/Blueprints/TopDownCharacter.TopDownCharacter_C|GetWeaponL _astop_down_character)) (Utilities|IsValid (Variables|/Game/TopDownBP/Blueprints/TopDownCharacter.TopDownCharacter_C|GetWeaponR _astop_down_character)))
        (goto _label)))))

(fn CheckFreeLine
  (params (Pawn :type Top%20Down%20Character%20Object%20Reference) (GridCell :type Grid%20Cell%20BP%20Object%20Reference))
  (bind _outhits (Class|KismetSystemLibrary|LineTraceMultiNEW (Transformation|GetActorLocation Pawn) (Transformation|GetActorLocation GridCell) "TraceTypeQuery1" false (Utilities|Array|MakeArray Pawn) "None" true "(R=1.000000,G=0.000000,B=0.000000,A=1.000000)" "(R=0.000000,G=1.000000,B=0.000000,A=1.000000)" 2.0))
  (bind _array_element (Utilities|Array|ForEachLoopwithBreak _outhits :!label _label)
    (:LoopBody
      (Utilities|Casting|CastToGridCell_BP (.HitActor (Collision|BreakHitResult _array_element))
        (:then
          (LocalVariables|SetFreeLine true))
        (:CastFailed
          (LocalVariables|SetFreeLine false)
          (goto _label Break))))
    (:Completed
      (return (LocalVariables|GetFreeLine)))))

(fn SpawnFireonCell
  (Variables|Default|SetFire true)
  (bind _returnvalue (Game|SpawnActorfromClass "/Game/Game/Code/Fire_BP.Fire_BP_C" (Math|Transform|MakeTransform (Transformation|GetActorLocation) "0, 0, 0" "6.000000,6.000000,6.000000") "Undefined" 0 0))
  (Variables|/Game/Game/Code/Fire_BP.Fire_BP_C|SetX _returnvalue (Variables|Default|GetX))
  (Variables|/Game/Game/Code/Fire_BP.Fire_BP_C|SetY _returnvalue (Variables|Default|GetY))
  (Variables|/Game/Game/Code/Fire_BP.Fire_BP_C|SetGridCell _returnvalue self)
  (return _returnvalue))