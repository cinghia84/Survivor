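; ItemsBox_BP is a clickable storage container that holds items and opens an item menu.
; Hovering its Box component swaps the mesh to a highlight material and restores the barrel material afterward.
; A click that passes a DistanceTrace check from the player pawn stops movement, initializes an ItemsBoxMenu widget with this box and pauses the game.
; StorageSpaceFree computes remaining capacity from Space, counting Items2Space entries as two slots each.
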(event OnBeginCursorOver(Box)
  (params (TouchedComponent :type Primitive%20Component%20Object%20Reference))
  (Rendering|Material|SetMaterial (Variables|Default|GetStaticMesh) 0 "/Game/Game/Code/MaterialHighlight/M_Highlight.M_Highlight"))

(event OnEndCursorOver(Box)
  (params (TouchedComponent :type Primitive%20Component%20Object%20Reference))
  (Rendering|Material|SetMaterial (Variables|Default|GetStaticMesh) 0 "/Game/InfinityBladeGrassLands/Environments/Breakables/Materials/M_Breakables_Barrels.M_Breakables_Barrels"))

(event OnClicked(Box)
  (params (TouchedComponent :type Primitive%20Component%20Object%20Reference) (ButtonPressed :type Key%20Structure :default "AnyKey"))
  (bind _returnvalue (Game|GetPlayerController 0))
  (bind _returnvalue_2 (CallFunction|DistanceTrace (Pawn|GetControlledPawn _returnvalue) self "ObjectTypeQuery24"))
  (if _returnvalue_2
    (AI|Navigation|StopMovement _returnvalue)
    (bind _returnvalue_3 (UserInterface|CreateWidget "/Game/Game/Menu/ItemsBoxMenu.ItemsBoxMenu_C"))
    (UserInterface|Viewport|AddtoViewport _returnvalue_3 0)
    (Variables|/Game/Game/Menu/ItemsBoxMenu.ItemsBoxMenu_C|SetItemsBox _returnvalue_3 self)
    (Default|Init _returnvalue_3)
    (Game|SetGamePaused true)))

(event EventBeginPlay)

(event Collision|EventActorBeginOverlap
  (params (OtherActor :type Actor%20Object%20Reference)))

(event EventTick
  (params (DeltaSeconds :type Float%20%28single-precision%29)))

(fn ConstructionScript)

(fn StorageSpaceFree
  (return (- (- (Variables|Default|GetSpace) (Utilities|Array|Length (Variables|Default|GetItems))) (* (Utilities|Array|Length (Variables|Default|GetItems2Space)) 2))))