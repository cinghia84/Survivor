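; Generic 3x3 room actor with modular walls, a door wall and a roof, scaled up threefold by its construction script.
; On BeginPlay it destroys any wall or door-wall component that is not visible, so component visibility determines the room's layout.
; A SetRoofVisibility event feeds the roof visibility value into the roof's hidden-in-game state, propagating it to child components.
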(event EventBeginPlay
  (for _array_element (Utilities|Array|MakeArray (Variables|Default|GetWall3) (Variables|Default|GetWall5) (Variables|Default|GetWall6) (Variables|Default|GetWall7) (Variables|Default|GetWall0) (Variables|Default|GetWall2) (Variables|Components|GetWall1) (Variables|Components|GetWall4) (Variables|Default|GetWall8) (Variables|Default|GetWall9) (Variables|Default|GetWall10) (Variables|Default|GetWall_Door))
    (if (not (Variables|/Script/Engine.SceneComponent|GetbVisible _array_element))
      (Components|DestroyComponent _array_element))))

(event Collision|EventActorBeginOverlap
  (params (OtherActor :type Actor%20Object%20Reference)))

(event EventSetRoofVisibility
  (bind _returnvalue (CallFunction|RoofVisibility self))
  (Development|SetHiddeninGame (Variables|Default|GetRoof) _returnvalue true))

(fn ConstructionScript
  (Transformation|SetActorScale3D "3.000000,3.000000,3.000000"))