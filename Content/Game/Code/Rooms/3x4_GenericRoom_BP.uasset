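; Generic 3x4 room actor built from wall, window, door and roof components.
; On BeginPlay it destroys any listed wall, window or door component that is not visible, so the visibility flag selects each instance's layout.
; A SetRoofVisibility event passes the result of RoofVisibility to the roof's hidden-in-game state, propagating to its children.
; The construction script only runs the parent's.
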(event EventBeginPlay
  (for _array_element (Utilities|Array|MakeArray (Variables|Default|GetWall4) (Variables|Default|GetWall5) (Variables|Default|GetWall6) (Variables|Default|GetWall7) (Variables|Default|GetWall0) (Variables|Default|GetWall2) (Variables|Default|GetWall3) (Variables|Default|GetWall1) (Variables|Default|GetWall8) (Variables|Default|GetWindow1) (Variables|Default|GetWindow2) (Variables|Default|GetWall_Door_BP) (Variables|Default|GetWindow3) (Variables|Default|GetWall9))
    (if (not (Variables|/Script/Engine.SceneComponent|GetbVisible _array_element))
      (Components|DestroyComponent _array_element))))

(event Collision|EventActorBeginOverlap
  (params (OtherActor :type Actor%20Object%20Reference)))

(event EventSetRoofVisibility
  (bind _returnvalue (CallFunction|RoofVisibility self))
  (Development|SetHiddeninGame (Variables|Default|GetRoof) _returnvalue true))

(fn ConstructionScript
  (|CallParentFunction))