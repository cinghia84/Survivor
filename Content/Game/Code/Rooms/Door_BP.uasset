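; Door actor that acts as a barricade, halting zombies that reach it.
; When a zombie begins overlapping its Box, it stops that zombie's AI movement if the door is whole or barricaded.
; While barricaded, Tick keeps stopping every overlapping zombie; once the barricade flag is false, Tick destroys the door, regardless of whether it is whole.
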(event OnComponentBeginOverlap(Box)
  (params (OverlappedComponent :type Primitive%20Component%20Object%20Reference) (OtherActor :type Actor%20Object%20Reference) (OtherComp :type Primitive%20Component%20Object%20Reference) (OtherBodyIndex :type Integer) (bFromSweep :type Boolean) (SweepResult :type Hit%20Result%20Structure%20%28by%20ref%29))
  (bind _aszombie_bp (Utilities|Casting|CastToZombie_BP OtherActor))
  (bind _returnvalue (AI|GetAIController _aszombie_bp))
  (if (or (Variables|Default|GetisWhole) (Variables|Default|GetisBarricade))
    (AI|Navigation|StopMovement _returnvalue)))

(event EventBeginPlay)

(event Collision|EventActorBeginOverlap
  (params (OtherActor :type Actor%20Object%20Reference)))

(event EventTick
  (params (DeltaSeconds :type Float%20%28single-precision%29))
  (if (Variables|Default|GetisBarricade)
    (for _array_element (Collision|GetOverlappingActors (Variables|Default|GetBox) "/Game/Characters/Zombie/Zombie_BP.Zombie_BP_C" :!class /Script/Engine.PrimitiveComponent)
      (bind _aszombie_bp (Utilities|Casting|CastToZombie_BP _array_element))
      (bind _returnvalue (AI|GetAIController _aszombie_bp))
      (AI|Navigation|StopMovement _returnvalue))
    (else
      (Actor|DestroyActor))))

(fn ConstructionScript)