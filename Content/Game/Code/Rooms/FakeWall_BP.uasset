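; FakeWall_BP is a clickable fake wall that can be replaced by a wooden barricade.
; Hovering its click box swaps in a highlight material and restores the original on exit.
; Clicking stops the player pawn and, if a distance trace passes, opens a WallMenu bound to this wall.
; The Barricade event spawns a rescaled, pine-textured Wall_BP flagged as a clickable barricade in its place, then destroys itself.
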(event OnBeginCursorOver(ClickBox)
  (params (TouchedComponent :type Primitive%20Component%20Object%20Reference))
  (bind _staticmesh (Variables|Default|GetStaticMesh))
  (Variables|Default|SetOldMaterial (Rendering|Material|GetMaterial _staticmesh 0))
  (Rendering|Material|SetMaterial _staticmesh 0 "/Game/Game/Code/MaterialHighlight/M_Highlight.M_Highlight"))

(event OnEndCursorOver(ClickBox)
  (params (TouchedComponent :type Primitive%20Component%20Object%20Reference))
  (Rendering|Material|SetMaterial (Variables|Default|GetStaticMesh) 0 (Variables|Default|GetOldMaterial)))

(event OnClicked(ClickBox)
  (params (TouchedComponent :type Primitive%20Component%20Object%20Reference) (ButtonPressed :type Key%20Structure :default "AnyKey"))
  (bind _returnvalue (Game|Player|GetPlayerPawn 0))
  (Class|NavMovementComponent|StopActiveMovement (Pawn|GetMovementComponent _returnvalue))
  (bind _returnvalue_2 (CallFunction|DistanceTrace _returnvalue self "ObjectTypeQuery10"))
  (if _returnvalue_2
    (bind _returnvalue_3 (UserInterface|CreateWidget "/Game/Game/Menu/WallMenu.WallMenu_C"))
    (UserInterface|Viewport|AddtoViewport _returnvalue_3 0)
    (Default|MoveandSet :self _returnvalue_3 :Wall self)))

(event Custom|Barricade
  (bind _self self)
  (bind _returnvalue (Game|SpawnActorfromClass "/Game/Game/Code/Rooms/Wall_BP.Wall_BP_C" (Transformation|GetActorTransform _self) "AlwaysSpawn" 0 0))
  (Transformation|SetActorScale3D _returnvalue "1.000000,1.400000,1.200000")
  (Rendering|Material|SetMaterial (Variables|/Game/Game/Code/Rooms/GenericWall_BP.GenericWall_BP_C|GetWallMesh _returnvalue) 0 "/Game/StarterContent/Materials/M_Wood_Pine.M_Wood_Pine")
  (Variables|/Game/Game/Code/Rooms/GenericWall_BP.GenericWall_BP_C|SetIsBarricade _returnvalue true)
  (Variables|/Game/Game/Code/Rooms/GenericWall_BP.GenericWall_BP_C|SetisClickable _returnvalue true)
  (Actor|DestroyActor _self))

(event EventBeginPlay)

(event EventTick
  (params (DeltaSeconds :type Float%20%28single-precision%29)))

(fn ConstructionScript)