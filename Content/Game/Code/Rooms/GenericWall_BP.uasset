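; GenericWall_BP is a clickable room wall that opens a WallMenu widget for that wall.
; Clicking stops the player's movement and removes any open WallMenu widgets.
; If the TopDownCharacter's sphere overlaps the wall's Box, it creates a new menu bound to this wall and pauses the game.
; Cursor hover swaps the mesh to a highlight material and restores the saved one on exit.
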(event OnBeginCursorOver(ClickBox)
  (params (TouchedComponent :type Primitive%20Component%20Object%20Reference))
  (bind _wallmesh (Variables|Default|GetWallMesh))
  ;[1 1 1] WallHighlight
  (Variables|Default|SetOldMaterial (Rendering|Material|GetMaterial _wallmesh 0))
  (Rendering|Material|SetMaterial _wallmesh 0 "/Game/Game/Code/MaterialHighlight/M_Highlight.M_Highlight"))

(event OnEndCursorOver(ClickBox)
  (params (TouchedComponent :type Primitive%20Component%20Object%20Reference))
  ;[1 1 1] WallHighlight
  (Rendering|Material|SetMaterial (Variables|Default|GetWallMesh) 0 (Variables|Default|GetOldMaterial)))

(event OnClicked(ClickBox)
  (params (TouchedComponent :type Primitive%20Component%20Object%20Reference) (ButtonPressed :type Key%20Structure :default "AnyKey"))
  (bind _returnvalue (Game|Player|GetPlayerPawn 0))
  (Class|NavMovementComponent|StopActiveMovement (Pawn|GetMovementComponent _returnvalue))
  (bind _foundwidgets (Widget|GetAllWidgetsOfClass "/Game/Game/Menu/WallMenu.WallMenu_C" true))
  (for _array_element _foundwidgets
    (Widget|RemovefromParent _array_element))
  (bind _astop_down_character (Utilities|Casting|CastToTopDownCharacter _returnvalue))
  (if (Class|PrimitiveComponent|IsOverlappingComponent (Variables|/Game/TopDownBP/Blueprints/TopDownCharacter.TopDownCharacter_C|GetSphere _astop_down_character) (Variables|Default|GetBox))
    (bind _returnvalue_2 (UserInterface|CreateWidget "/Game/Game/Menu/WallMenu.WallMenu_C"))
    (UserInterface|Viewport|AddtoViewport _returnvalue_2 0)
    (Default|MoveandSet :self _returnvalue_2 :Wall self)
    (Game|SetGamePaused true)))

(event EventBeginPlay)

(fn ConstructionScript)