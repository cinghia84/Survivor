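; Box volume actor that spawns the player pawns inside a start area when SpawnPlayers is called.
; For each of the game mode's NumPlayer, it picks a random point at the box's top and resolves ground through HitGroundLocation, retrying without limit until it hits.
; It spawns a random class from PawnTypeArray there, registers the TopDownCharacter in the game mode's PawnArray and assigns a generated name.
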(event Custom|SpawnPlayers
  (bind _pawntypearray (Variables|Default|GetPawnTypeArray))
  (bind _box (Variables|Default|GetBox))
  (bind _returnvalue (Components|Box|GetScaledBoxExtent _box))
  (bind (_x _y _z) (Math|Vector|BreakVector _returnvalue))
  (bind _astop_down_game_mode (Utilities|Casting|CastToTopDownGameMode (Game|GetGameMode)))
  (for _index (range 0 (- (Variables|/Game/TopDownBP/Blueprints/TopDownGameMode.TopDownGameMode_C|GetNumPlayer _astop_down_game_mode) 1))
    (bind (_return_value _hit) (CallFunction|HitGroundLocation (+ (Math|Vector|MakeVector (Math|Random|RandomFloatinRange (* _x -1.0) _x) (Math|Random|RandomFloatinRange (* _y -1.0) _y) _z) (Transformation|GetActorLocation self)) 1.5e+02 (Utilities|Array|MakeArray 0) :!label _label))
    (if _hit
      (bind _returnvalue_2 (Game|SpawnActorfromClass (Utilities|Array|Get(acopy) _pawntypearray (Math|Random|RandomIntegerinRange 0 (Utilities|Array|LastIndex _pawntypearray))) (Math|Conversions|ToTransform(Vector) _return_value) "AdjustIfPossibleButAlwaysSpawn" 0 0))
      (bind _astop_down_character (Utilities|Casting|CastToTopDownCharacter _returnvalue_2))
      (Utilities|Array|Add (Variables|/Game/TopDownBP/Blueprints/TopDownGameMode.TopDownGameMode_C|GetPawnArray _astop_down_game_mode) _astop_down_character)
      (bind _row (CallFunction|CreatePawnName))
      (Variables|/Game/TopDownBP/Blueprints/TopDownCharacter.TopDownCharacter_C|SetPlayerName _astop_down_character (.Name (Utilities|Struct|BreakNamesStruct _row)))
      (else
        (goto _label)))))

(event Collision|EventActorBeginOverlap
  (params (OtherActor :type Actor%20Object%20Reference)))

(fn ConstructionScript)