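; Wall window actor for rooms that can switch between a glass window and a wooden barricade.
; Every Tick reapplies the look from the IsBarricade flag, swapping the Window material between pine and glass and toggling the barricade and window sprites.
; When barricaded, WallMesh blocks all channels; otherwise it ignores them, except Visibility, which it overlaps.
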(event EventBeginPlay)

(event Collision|EventActorBeginOverlap
  (params (OtherActor :type Actor%20Object%20Reference)))

(event EventTick
  (params (DeltaSeconds :type Float%20%28single-precision%29))
  (bind _barricadesprite (Variables|Default|GetBarricadeSprite))
  (bind _window (Variables|Default|GetWindow))
  (bind _wallmesh (Variables|Default|GetWallMesh))
  (bind _windowsprite (Variables|Default|GetWindowSprite))
  (if (Variables|Default|GetIsBarricade)
    (Rendering|Material|SetMaterial _window 0 "/Game/StarterContent/Materials/M_Wood_Pine.M_Wood_Pine")
    (Collision|SetCollisionResponsetoAllChannels _wallmesh "ECR_Block")
    (Collision|SetCollisionResponsetoChannel _wallmesh "ECC_Visibility" "ECR_Block")
    (Development|SetHiddeninGame _barricadesprite false false)
    (Development|SetHiddeninGame _windowsprite true false)
    (else
      (Rendering|Material|SetMaterial _window 0 "/Game/StarterContent/Materials/M_Glass.M_Glass")
      (Collision|SetCollisionResponsetoAllChannels _wallmesh "ECR_Ignore")
      (Collision|SetCollisionResponsetoChannel _wallmesh "ECC_Visibility" "ECR_Overlap")
      (Development|SetHiddeninGame _barricadesprite true false)
      (Development|SetHiddeninGame _windowsprite false false))))

(fn ConstructionScript
  (|CallParentFunction))