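; Window trigger box that offers the player character a menu to move to its linked BoxDestination.
; Each Tick checks whether player 0's character and any Ladder_BP overlap the box.
; During a turn, a ladder brings up StairsMenu; without one, upper floors get JumpWindowsMenu, both targeting the destination at fixed height.
; Menus close when the player leaves or the turn ends; a separate helper reports whether characters share the floor.
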(event EventBeginPlay)

(event Collision|EventActorBeginOverlap
  (params (OtherActor :type Actor%20Object%20Reference)))

(event EventTick
  (params (DeltaSeconds :type Float%20%28single-precision%29))
  (bind _boxdestination (Variables|Default|GetBoxDestination))
  (bind _boxdestination_2 (Variables|Default|GetBoxDestination))
  (bind _returnvalue (Transformation|GetActorLocation _boxdestination_2))
  (bind _returnvalue_2 (Transformation|GetActorLocation _boxdestination))
  (bind (_x _y) (Math|Vector|BreakVector _returnvalue))
  (bind (_x_2 _y_2) (Math|Vector|BreakVector _returnvalue_2))
  (bind _return (CallFunction|CheckPawnOverlap))
  (bind _return_value (CallFunction|CheckOverlapLadder))
  (if _return_value
    (Utilities|IsValid _return
      (:Is%20Valid
        (bind _astop_down_game_mode (Utilities|Casting|CastToTopDownGameMode (Game|GetGameMode)))
        (if (Variables|/Game/TopDownBP/Blueprints/TopDownGameMode.TopDownGameMode_C|GetDuringTurn _astop_down_game_mode)
          (Utilities|IsValid (Variables|Default|GetWidget)
            (:Is%20Not%20Valid
              (bind _returnvalue_3 (UserInterface|CreateWidget "/Game/Game/Menu/StairsMenu.StairsMenu_C"))
              (UserInterface|Viewport|AddtoViewport _returnvalue_3 0)
              (Variables|Default|SetWidget _returnvalue_3)
              (Variables|/Game/Game/Menu/StairsMenu.StairsMenu_C|SetTargetDestination _returnvalue_3 (Math|Vector|MakeVector _x_2 _y_2 118.0))))
          (else
            (Utilities|IsValid (Variables|Default|GetWidget)
              (:Is%20Valid
                (Widget|RemovefromParent (Variables|Default|GetWidget) :!label _label)
                (Variables|Default|SetWidget 0))))))
      (:Is%20Not%20Valid
        (Utilities|IsValid (Variables|Default|GetWidget)
          (:Is%20Valid
            (goto _label)))))
    (elif (> (Variables|Default|GetFloor) 0)
      (Utilities|IsValid _return
        (:Is%20Valid
          (bind _astop_down_game_mode_2 (Utilities|Casting|CastToTopDownGameMode (Game|GetGameMode)))
          (if (Variables|/Game/TopDownBP/Blueprints/TopDownGameMode.TopDownGameMode_C|GetDuringTurn _astop_down_game_mode_2)
            (Utilities|IsValid (Variables|Default|GetWidgetJump)
              (:Is%20Not%20Valid
                (bind _returnvalue_4 (UserInterface|CreateWidget "/Game/Game/Menu/JumpWindowsMenu.JumpWindowsMenu_C"))
                (UserInterface|Viewport|AddtoViewport _returnvalue_4 0)
                (Variables|Default|SetWidgetJump _returnvalue_4)
                (Variables|/Game/Game/Menu/JumpWindowsMenu.JumpWindowsMenu_C|SetTargetDestination _returnvalue_4 (Math|Vector|MakeVector _x _y 118.0))))
            (else
              (Utilities|IsValid (Variables|Default|GetWidgetJump)
                (:Is%20Valid
                  (Widget|RemovefromParent (Variables|Default|GetWidgetJump) :!label _label_2)
                  (Variables|Default|SetWidgetJump 0))))))
        (:Is%20Not%20Valid
          (Utilities|IsValid (Variables|Default|GetWidgetJump)
            (:Is%20Valid
              (goto _label_2))))))))

(fn ConstructionScript)

(fn CheckPawnOverlap
  (bind _astop_down_character (Utilities|Casting|CastToTopDownCharacter (Game|Player|GetPlayerPawn 0)))
  (bind _array_element (Utilities|Array|ForEachLoopwithBreak (Collision|GetOverlappingActors (Variables|Default|GetBox) "/Game/TopDownBP/Blueprints/TopDownCharacter.TopDownCharacter_C" :!class /Script/Engine.PrimitiveComponent) :!label _label)
    (:LoopBody
      (bind _astop_down_character_2 (Utilities|Casting|CastToTopDownCharacter _array_element))
      (if (== _astop_down_character_2 _astop_down_character)
        (LocalVariables|SetPawn _astop_down_character_2)
        (goto _label Break)))
    (:Completed
      (return (LocalVariables|GetPawn)))))

(fn CheckPawnonSameFloor
  (params (Zombie :type Zombie%20BP%20Object%20Reference))
  (bind _outactors (Actor|GetAllActorsOfClass "/Game/TopDownBP/Blueprints/TopDownCharacter.TopDownCharacter_C"))
  (for _array_element _outactors
    (if (== (Variables|/Game/TopDownBP/Blueprints/TopDownCharacter.TopDownCharacter_C|GetFloor _array_element) (Variables|Default|GetFloor))
      (Math|Integer|IncrementInt (LocalVariables|GetPawnOnFloor))))
  (if (> (LocalVariables|GetPawnOnFloor) 0)
    (return true)
    (else
      (return false))))

(fn CheckOverlapLadder
  (return (> (Utilities|Array|Length (Collision|GetOverlappingActors (Variables|Default|GetBox) "/Game/Game/Images/Objs/Blueprint/ladder_BP.ladder_BP_C" :!class /Script/Engine.PrimitiveComponent)) 0)))