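; Room actor that scatters Zombie_BP enemies across its box area, then destroys itself.
; Spawning runs on BeginPlay, and the same logic is also wired to box overlap by a TopDownCharacter.
; The zombie count scales with the box's larger horizontal extent.
; Each attempt picks a random point in the box, spawns only if HitGroundLocation finds ground, and gives the zombie a random yaw.
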(event OnComponentBeginOverlap(Box)
  (params (OverlappedComponent :type Primitive%20Component%20Object%20Reference) (OtherActor :type Actor%20Object%20Reference) (OtherComp :type Primitive%20Component%20Object%20Reference) (OtherBodyIndex :type Integer) (bFromSweep :type Boolean) (SweepResult :type Hit%20Result%20Structure%20%28by%20ref%29))
  (bind _box (Variables|Default|GetBox))
  (bind _box_2 (Variables|Default|GetBox))
  (bind _returnvalue (Components|Box|GetScaledBoxExtent _box_2))
  (bind _returnvalue_2 (Components|Box|GetScaledBoxExtent _box))
  (bind (_x _y) (Math|Vector|BreakVector _returnvalue_2))
  (bind (_x_2 _y_2) (Math|Vector|BreakVector _returnvalue))
  (Utilities|Casting|CastToTopDownCharacter OtherActor)
  (for _index (range 1 (Math|Float|Truncate (/ (Math|Float|Max(Float) _x _y) 1e+02)))
    (bind (_return_value _hit) (CallFunction|HitGroundLocation (+ (Math|Vector|MakeVector (Math|Random|RandomFloatinRange (* _x_2 -1.0) _x_2) (Math|Random|RandomFloatinRange (* _y_2 -1.0) _y_2) 118.0) (Transformation|GetActorLocation self)) 1.5e+02 (Utilities|Array|MakeArray 0)))
    (if _hit
      (bind _returnvalue_3 (Game|SpawnActorfromClass "/Game/Characters/Zombie/Zombie_BP.Zombie_BP_C" (Math|Conversions|ToTransform(Vector) _return_value) "AlwaysSpawn" 0 0))
      (Transformation|SetActorRotation _returnvalue_3 (Math|Rotator|MakeRotator 0.0 0.0 (Math|Random|RandomFloatinRange -1.8e+02 1.8e+02)))))
  (Actor|DestroyActor))

(event EventBeginPlay
  (bind _box (Variables|Default|GetBox))
  (bind _box_2 (Variables|Default|GetBox))
  (bind _returnvalue (Components|Box|GetScaledBoxExtent _box_2))
  (bind _returnvalue_2 (Components|Box|GetScaledBoxExtent _box))
  (bind (_x _y) (Math|Vector|BreakVector _returnvalue_2))
  (bind (_x_2 _y_2) (Math|Vector|BreakVector _returnvalue))
  (for _index (range 1 (Math|Float|Truncate (/ (Math|Float|Max(Float) _x _y) 1e+02)))
    (bind (_return_value _hit) (CallFunction|HitGroundLocation (+ (Math|Vector|MakeVector (Math|Random|RandomFloatinRange (* _x_2 -1.0) _x_2) (Math|Random|RandomFloatinRange (* _y_2 -1.0) _y_2) 118.0) (Transformation|GetActorLocation self)) 1.5e+02 (Utilities|Array|MakeArray 0)))
    (if _hit
      (bind _returnvalue_3 (Game|SpawnActorfromClass "/Game/Characters/Zombie/Zombie_BP.Zombie_BP_C" (Math|Conversions|ToTransform(Vector) _return_value) "AlwaysSpawn" 0 0))
      (Transformation|SetActorRotation _returnvalue_3 (Math|Rotator|MakeRotator 0.0 0.0 (Math|Random|RandomFloatinRange -1.8e+02 1.8e+02)))))
  (Actor|DestroyActor))

(event Collision|EventActorBeginOverlap
  (params (OtherActor :type Actor%20Object%20Reference)))

(event EventTick
  (params (DeltaSeconds :type Float%20%28single-precision%29)))

(fn ConstructionScript)