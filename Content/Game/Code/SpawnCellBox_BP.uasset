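; SpawnCellBox_BP is a box-volume actor built to fill its area with a grid of GridCell_BP actors.
; Its logic derives start corner and cell counts from box extent and BlockSize, calls SpawnCell, copies the grid size to TopDownGameMode, then destroys itself.
; SpawnCell tags each cell with X/Y indices and registers it through AddCell.
; The setup chain is disconnected from BeginPlay, so it never runs as it stands.
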(event EventBeginPlay)

(event Collision|EventActorBeginOverlap
  (params (OtherActor :type Actor%20Object%20Reference)))

(event EventTick
  (params (DeltaSeconds :type Float%20%28single-precision%29)))

(fn ConstructionScript)

(fn SpawnCell
  (bind _blocksize (Variables|Default|GetBlockSize))
  (for _index (range 0 (- (Variables|Default|GetSizeY) 1)) ; Loop to spawn each block
    (for _index_2 (range 0 (- (Variables|Default|GetSizeX) 1))
      (bind _returnvalue (Game|SpawnActorfromClass "/Game/Game/Code/GridCell_BP.GridCell_BP_C" (Math|Conversions|ToTransform(Vector) (+ (Math|Vector|MakeVector (* _index_2 _blocksize) (* _index _blocksize) 0.0) (Variables|Default|GetStartLocation))) "AlwaysSpawn" 0 0)) ; Spawn a  block
      (bind _output_get (Variables|/Game/Game/Code/GridCell_BP.GridCell_BP_C|SetX _returnvalue _index_2))
      (bind _output_get_2 (Variables|/Game/Game/Code/GridCell_BP.GridCell_BP_C|SetY _returnvalue _index))
      (bind _astop_down_game_mode (Utilities|Casting|CastToTopDownGameMode (Game|GetGameMode)))
      (Default|AddCell _astop_down_game_mode (Utilities|Struct|MakeCellStruct _output_get _output_get_2 _returnvalue)))))