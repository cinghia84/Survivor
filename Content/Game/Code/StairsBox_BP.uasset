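; StairsBox_BP is a stairs trigger volume linking to a TargetDestination actor for players and zombies in a turn-based top-down game.
; Tick polls whether the player pawn overlaps the box during a turn, creating a StairsMenu with the destination or removing it otherwise.
; Zombies entering the box teleport to the destination if CanZombieWalk is set and no TopDownCharacter shares the stairs' Floor.
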(event OnComponentBeginOverlap(Box)
  (params (OverlappedComponent :type Primitive%20Component%20Object%20Reference) (OtherActor :type Actor%20Object%20Reference) (OtherComp :type Primitive%20Component%20Object%20Reference) (OtherBodyIndex :type Integer) (bFromSweep :type Boolean) (SweepResult :type Hit%20Result%20Structure%20%28by%20ref%29))
  (bind _aszombie_bp (Utilities|Casting|CastToZombie_BP OtherActor))
  (if (Variables|Default|GetCanZombieWalk)
    (bind _return (CallFunction|CheckPawnonSameFloor _aszombie_bp))
    (if (not _return)
      (Transformation|SetActorLocation _aszombie_bp (Transformation|GetActorLocation (Variables|Default|GetTargetDestination)) false true))))

(event EventBeginPlay)

(event Collision|EventActorBeginOverlap
  (params (OtherActor :type Actor%20Object%20Reference)))

(event EventTick
  (params (DeltaSeconds :type Float%20%28single-precision%29))
  (bind _return (CallFunction|CheckPawnOverlap))
  (Utilities|IsValid _return
    (:Is%20Valid
      (bind _astop_down_game_mode (Utilities|Casting|CastToTopDownGameMode (Game|GetGameMode)))
      (if (Variables|/Game/TopDownBP/Blueprints/TopDownGameMode.TopDownGameMode_C|GetDuringTurn _astop_down_game_mode)
        (Utilities|IsValid (Variables|Default|GetWidget)
          (:Is%20Not%20Valid
            (bind _returnvalue (UserInterface|CreateWidget "/Game/Game/Menu/StairsMenu.StairsMenu_C"))
            (UserInterface|Viewport|AddtoViewport _returnvalue 0)
            (Variables|Default|SetWidget _returnvalue)
            (Variables|/Game/Game/Menu/StairsMenu.StairsMenu_C|SetTargetDestination _returnvalue (Transformation|GetActorLocation (Variables|Default|GetTargetDestination)))))
        (else
          (Utilities|IsValid (Variables|Default|GetWidget)
            (:Is%20Valid
              (Widget|RemovefromParent (Variables|Default|GetWidget) :!label _label)
              (Variables|Default|SetWidget 0))))))
    (:Is%20Not%20Valid
      (Utilities|IsValid (Variables|Default|GetWidget)
        (:Is%20Valid
          (goto _label))))))

(fn ConstructionScript)

(fn CheckPawnOverlap
  (bind _astop_down_character (Utilities|Casting|CastToTopDownCharacter (Game|Player|GetPlayerPawn 0)))
  (bind _array_element (Utilities|Array|ForEachLoopwithBreak (Collision|GetOverlappingActors (Variables|Default|GetBox) "/Game/TopDownBP/Blueprints/TopDownCharacter.TopDownCharacter_C" :!class /Script/Engine.PrimitiveComponent) :!label _label)
    (:LoopBody
      (bind _astop_down_character_2 (Utilities|Casting|CastToTopDownCharacter _array_element))
      (if (== _astop_down_character_2 _astop_down_character)
        (LocalVariables|SetPawn _astop_down_character_2)
        (goto _label Break)))
    (:Completed
      (return (LocalVariables|GetPawn)))))

(fn CheckPawnonSameFloor
  (params (Zombie :type Zombie%20BP%20Object%20Reference))
  (bind _outactors (Actor|GetAllActorsOfClass "/Game/TopDownBP/Blueprints/TopDownCharacter.TopDownCharacter_C"))
  (for _array_element _outactors
    (if (== (Variables|/Game/TopDownBP/Blueprints/TopDownCharacter.TopDownCharacter_C|GetFloor _array_element) (Variables|Default|GetFloor))
      (Math|Integer|IncrementInt (LocalVariables|GetPawnOnFloor))))
  (if (> (LocalVariables|GetPawnOnFloor) 0)
    (return true)
    (else
      (return false))))