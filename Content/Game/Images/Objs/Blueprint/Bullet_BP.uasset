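; Bullet_BP is a clickable bullet object holding a random ammo count, rolled between set limits in the construction script.
; Clicking its Box stops the player pawn's movement, then runs a DistanceTrace between the pawn and the object.
; When the trace succeeds, it opens a BulletMenu widget and passes itself in as that menu's Object.
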(event OnClicked(Box)
  (params (TouchedComponent :type Primitive%20Component%20Object%20Reference) (ButtonPressed :type Key%20Structure :default "AnyKey"))
  (bind _returnvalue (Game|Player|GetPlayerPawn 0))
  (Class|NavMovementComponent|StopActiveMovement (Pawn|GetMovementComponent _returnvalue))
  (bind _returnvalue_2 (CallFunction|DistanceTrace _returnvalue self "ObjectTypeQuery20"))
  (if _returnvalue_2
    (bind _returnvalue_3 (UserInterface|CreateWidget "/Game/Game/Menu/BulletMenu.BulletMenu_C"))
    (UserInterface|Viewport|AddtoViewport _returnvalue_3 0)
    (Variables|/Game/Game/Menu/BulletMenu.BulletMenu_C|SetObject _returnvalue_3 self)))

(event EventBeginPlay)

(event Collision|EventActorBeginOverlap
  (params (OtherActor :type Actor%20Object%20Reference)))

(fn ConstructionScript
  (Variables|Default|SetAmmo (Math|Random|RandomIntegerinRange 1 6))
  (Transformation|SetActorScale3D "1.000000,1.000000,1.000000"))