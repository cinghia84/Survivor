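; Generator actor that offers an interaction menu when the player comes within its box trigger and displays its power state.
; Tick polls overlapping pawns, creating a GeneratorMenu linked to itself for the player during a turn and removing it otherwise.
; Overlap events also open the menu, only if the generator is neither started nor damaged, and remove it on exit.
; Each tick, SetTextOnVideo updates the message to powered, damaged or blank.
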(event OnComponentBeginOverlap(Box)
  (params (OverlappedComponent :type Primitive%20Component%20Object%20Reference) (OtherActor :type Actor%20Object%20Reference) (OtherComp :type Primitive%20Component%20Object%20Reference) (OtherBodyIndex :type Integer) (bFromSweep :type Boolean) (SweepResult :type Hit%20Result%20Structure%20%28by%20ref%29))
  (Utilities|Casting|CastToTopDownCharacter OtherActor)
  (if (and (not (Variables|Default|GetStarted)) (not (Variables|Default|GetDamaged)))
    (bind _returnvalue (UserInterface|CreateWidget "/Game/Game/Menu/GeneratorMenu.GeneratorMenu_C"))
    (UserInterface|Viewport|AddtoViewport _returnvalue 0)
    (Variables|/Game/Game/Menu/GeneratorMenu.GeneratorMenu_C|SetGenerator _returnvalue self)
    (Variables|Default|SetWidget _returnvalue)))

(event OnComponentEndOverlap(Box)
  (params (OverlappedComponent :type Primitive%20Component%20Object%20Reference) (OtherActor :type Actor%20Object%20Reference) (OtherComp :type Primitive%20Component%20Object%20Reference) (OtherBodyIndex :type Integer))
  (Utilities|Casting|CastToTopDownCharacter OtherActor)
  (Widget|RemovefromParent (Variables|Default|GetWidget)))

(event EventBeginPlay)

(event EventTick
  (params (DeltaSeconds :type Float%20%28single-precision%29))
  (Utilities|FlowControl|Sequence
    (:then_0
      (for _array_element (Collision|GetOverlappingActors (Variables|Default|GetBox) "/Script/Engine.Pawn" :!class /Script/Engine.PrimitiveComponent)
        (if (== (Game|Player|GetPlayerPawn 0) _array_element)
          (bind _astop_down_game_mode (Utilities|Casting|CastToTopDownGameMode (Game|GetGameMode)))
          (if (Variables|/Game/TopDownBP/Blueprints/TopDownGameMode.TopDownGameMode_C|GetDuringTurn _astop_down_game_mode)
            (Utilities|IsValid (Variables|Default|GetWidget)
              (:Is%20Not%20Valid
                (bind _returnvalue (UserInterface|CreateWidget "/Game/Game/Menu/GeneratorMenu.GeneratorMenu_C"))
                (UserInterface|Viewport|AddtoViewport _returnvalue 0)
                (Variables|/Game/Game/Menu/GeneratorMenu.GeneratorMenu_C|SetGenerator _returnvalue self)
                (Variables|Default|SetWidget _returnvalue)))
            (else
              (Utilities|IsValid (Variables|Default|GetWidget) :!label _label
                (:Is%20Valid
                  (Widget|RemovefromParent (Variables|Default|GetWidget))
                  (Variables|Default|SetWidget 0)))))
          (else
            (goto _label)))))
    (:then_1
      (CallFunction|SetTextonVideo))))

(fn ConstructionScript
  (Transformation|SetActorScale3D "2.000000,1.000000,2.000000"))

(fn SetTextonVideo
  (bind _message (Variables|Default|GetMessage))
  (if (Variables|Default|GetStarted)
    (Rendering|Components|TextRender|SetText _message (Utilities|Text|ToText(String) "Power On"))
    (elif (Variables|Default|GetDamaged)
      (Rendering|Components|TextRender|SetText _message (Utilities|Text|ToText(String) "Damaged"))
      (else
        (Rendering|Components|TextRender|SetText _message (Utilities|Text|ToText(String) " "))))))