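; Shotgun object Blueprint that takes on a randomly chosen look from its sprite and texture arrays.
; The construction script rolls one index within the TextureArray bounds, stores that texture in Texture, and applies the SpriteArray entry at the same index to the PaperSprite.
; It then calls the parent construction script, so Texture is set before inherited setup runs.
; The event graph holds only disabled placeholder events.
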(event EventBeginPlay)

(event Collision|EventActorBeginOverlap
  (params (OtherActor :type Actor%20Object%20Reference)))

(event EventTick
  (params (DeltaSeconds :type Float%20%28single-precision%29)))

(fn ConstructionScript
  (bind _texturearray (LocalVariables|GetTextureArray))
  (bind _output_get (LocalVariables|SetIndex (Math|Random|RandomIntegerinRange 0 (Utilities|Array|LastIndex _texturearray))))
  (Variables|Default|SetTexture (Utilities|Array|Get(acopy) _texturearray _output_get))
  (Rendering|Components|Sprite|SetSprite (Variables|Default|GetPaperSprite) (Utilities|Array|Get(acopy) (LocalVariables|GetSpriteArray) _output_get))
  (|CallParentFunction))