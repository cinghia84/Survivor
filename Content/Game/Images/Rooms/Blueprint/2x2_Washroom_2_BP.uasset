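; Washroom room actor that handles a player search, which can yield a first aid pickup.
; Search branches on its value: cases 1 to 4 only call DrawTextOnScreen with an enum message.
; Any other value spawns First_aid_BP a random short distance ahead of the player, placed and angled via a ground-hit helper, then passes it to SearchRoomResult.
; The construction script forces a uniform triple scale on the room.
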(event EventBeginPlay)

(event Collision|EventActorBeginOverlap
  (params (OtherActor :type Actor%20Object%20Reference)))

(event EventTick
  (params (DeltaSeconds :type Float%20%28single-precision%29)))

(event EventSearch
  (params (Value :type Integer))
  (bind _returnvalue (Game|Player|GetPlayerPawn 0))
  (bind (_return_value _hit _rotator) (CallFunction|HitGroundLocation (+ (Transformation|GetActorLocation _returnvalue) (* (Transformation|GetActorForwardVector _returnvalue) (Math|Random|RandomFloatinRange 5e+01 1.5e+02))) 2.0 (Utilities|Array|MakeArray 0)))
  (switch int Value
    (:Default
      (bind _returnvalue_2 (Game|SpawnActorfromClass "/Game/Game/Images/Objs/Blueprint/first_aid_BP.first_aid_BP_C" (Math|Transform|MakeTransform _return_value (Math|Rotator|MakeRotator (.Roll (Math|Rotator|BreakRotator _rotator)) 0.0 (.Yaw (Math|Rotator|BreakRotator _rotator))) "1.000000,1.000000,1.000000") "Undefined" 0 0))
      (CallFunction|SearchRoomResult _returnvalue_2))
    (:1
      (CallFunction|DrawTextonScreen "NewEnumerator1" :!label _label))
    (:2
      (goto _label))
    (:3
      (goto _label))
    (:4
      (goto _label))))

(fn ConstructionScript
  (Transformation|SetActorScale3D "3.000000,3.000000,3.000000"))