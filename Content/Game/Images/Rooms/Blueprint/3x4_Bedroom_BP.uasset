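; Bedroom room Blueprint whose Search event spawns either a loot item or a zombie based on the passed value.
; Shotgun, torch or hammer pickups land on traced ground ahead of the player and are passed to SearchRoomResult.
; Zombies spawn on ground at a random offset from the room actor, followed by a DrawTextOnScreen call.
; The construction script triples the actor's scale.
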(event EventBeginPlay)

(event Collision|EventActorBeginOverlap
  (params (OtherActor :type Actor%20Object%20Reference)))

(event EventTick
  (params (DeltaSeconds :type Float%20%28single-precision%29)))

(event EventSearch
  (params (Value :type Integer))
  (bind _returnvalue (Math|Random|RandomFloatinRange 5e+01 1.5e+02))
  (bind _returnvalue_2 (Game|Player|GetPlayerPawn 0))
  (bind _array (Utilities|Array|MakeArray 0))
  (bind _self self)
  (bind _returnvalue_3 (Transformation|GetActorLocation _self))
  (bind (_x _y) (Math|Vector|BreakVector _returnvalue_3))
  (bind _return_value (CallFunction|HitGroundLocation (Math|Vector|MakeVector (+ _x _returnvalue) (+ _y _returnvalue) 0.0) 2e+02 _array))
  (bind (_return_value_2 _hit _rotator) (CallFunction|HitGroundLocation (+ (Transformation|GetActorLocation _returnvalue_2) (* (Transformation|GetActorForwardVector _returnvalue_2) (Math|Random|RandomFloatinRange 5e+01 1.5e+02))) 2.0 _array))
  (switch int Value
    (:Default
      (bind _returnvalue_4 (Game|SpawnActorfromClass "/Game/Game/Images/Objs/Blueprint/shotgun_BP.shotgun_BP_C" (Math|Transform|MakeTransform _return_value_2 (Math|Rotator|MakeRotator (.Roll (Math|Rotator|BreakRotator _rotator)) 0.0 (.Yaw (Math|Rotator|BreakRotator _rotator))) "1.000000,1.000000,1.000000") "Undefined" 0 0))
      (CallFunction|SearchRoomResult _returnvalue_4))
    (:1
      (Game|SpawnActorfromClass "/Game/Characters/Zombie/Zombie_BP.Zombie_BP_C" (Math|Conversions|ToTransform(Vector) _return_value) "AdjustIfPossibleButAlwaysSpawn" 0 0 :!label _label)
      (CallFunction|DrawTextonScreen "NewEnumerator0"))
    (:2
      (goto _label))
    (:3
      (bind _returnvalue_5 (Game|SpawnActorfromClass "/Game/Game/Images/Objs/Blueprint/torch_BP.torch_BP_C" (Math|Transform|MakeTransform _return_value_2 (Math|Rotator|MakeRotator (.Roll (Math|Rotator|BreakRotator _rotator)) 0.0 (.Yaw (Math|Rotator|BreakRotator _rotator))) "1.000000,1.000000,1.000000") "Undefined" 0 0 :!label _label_2))
      (CallFunction|SearchRoomResult _returnvalue_5))
    (:4
      (goto _label_2))
    (:5
      (bind _returnvalue_6 (Game|SpawnActorfromClass "/Game/Game/Images/Objs/Blueprint/hammer_BP.hammer_BP_C" (Math|Transform|MakeTransform _return_value_2 (Math|Rotator|MakeRotator (.Roll (Math|Rotator|BreakRotator _rotator)) 0.0 (.Yaw (Math|Rotator|BreakRotator _rotator))) "1.000000,1.000000,1.000000") "Undefined" 0 0))
      (CallFunction|SearchRoomResult _returnvalue_6))))

(fn ConstructionScript
  (Transformation|SetActorScale3D "3.000000,3.000000,3.000000"))