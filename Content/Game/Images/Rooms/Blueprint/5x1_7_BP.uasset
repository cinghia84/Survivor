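; A room Blueprint, apparently a 5x1 layout variant, with two wall-door components and a roof.
; On BeginPlay it destroys whichever of WallDoor1 and WallDoor2 is not visible, so only visible ones remain.
; SetRoofVisibility passes the result of RoofVisibility to the Roof's hidden-in-game state, propagated to its children.
; The construction script only calls its parent.
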(event EventBeginPlay
  (for _array_element (Utilities|Array|MakeArray (Variables|Default|GetWallDoor1) (Variables|Default|GetWallDoor2))
    (if (not (Variables|/Script/Engine.SceneComponent|GetbVisible _array_element))
      (Components|DestroyComponent _array_element))))

(event Collision|EventActorBeginOverlap
  (params (OtherActor :type Actor%20Object%20Reference)))

(event EventTick
  (params (DeltaSeconds :type Float%20%28single-precision%29))
  (|CallParentFunction 0.0))

(event EventSetRoofVisibility
  (bind _returnvalue (CallFunction|RoofVisibility self))
  (Development|SetHiddeninGame (Variables|Default|GetRoof) _returnvalue true))

(fn ConstructionScript
  (|CallParentFunction))