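; Bedroom room Blueprint (5x5) that supplies the loot outcomes when the room is searched.
; Search switches on the passed Value to spawn a bat, stick, guitar or food pickup, or only call an on-screen text display with empty text.
; Items spawn at a random short distance in front of the player, snapped to the ground via HitGroundLocation, then pass to SearchRoomResult.
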(event Custom|Search
  (params (Value :type Integer))
  (bind _returnvalue (Game|Player|GetPlayerPawn 0))
  (bind (_return_value _hit _rotator) (CallFunction|HitGroundLocation (+ (Transformation|GetActorLocation _returnvalue) (* (Transformation|GetActorForwardVector _returnvalue) (Math|Random|RandomFloatinRange 5e+01 1.5e+02))) 2.0 (Utilities|Array|MakeArray 0)))
  (switch int Value
    (:Default
      (bind _returnvalue_2 (Game|SpawnActorfromClass "/Game/Game/Images/Objs/Blueprint/bat_BP.bat_BP_C" (Math|Transform|MakeTransform _return_value (Math|Rotator|MakeRotator (.Roll (Math|Rotator|BreakRotator _rotator)) 0.0 (.Yaw (Math|Rotator|BreakRotator _rotator))) "1.300000,1.300000,1.300000") "Undefined" 0 0))
      (CallFunction|SearchRoomResult _returnvalue_2))
    (:1
      (CallFunction|DrawTextonScreen "NewEnumerator1" :!label _label))
    (:2
      (goto _label))
    (:3
      (bind _returnvalue_3 (Game|SpawnActorfromClass "/Game/Game/Images/Objs/Blueprint/stick_BP.stick_BP_C" (Math|Transform|MakeTransform _return_value (Math|Rotator|MakeRotator (.Roll (Math|Rotator|BreakRotator _rotator)) 0.0 (.Yaw (Math|Rotator|BreakRotator _rotator))) "1.300000,1.300000,1.300000") "Undefined" 0 0 :!label _label_2))
      (CallFunction|SearchRoomResult _returnvalue_3))
    (:4
      (goto _label_2))
    (:5
      (bind _returnvalue_4 (Game|SpawnActorfromClass "/Game/Game/Images/Objs/Blueprint/guitar_BP.guitar_BP_C" (Math|Transform|MakeTransform _return_value (Math|Rotator|MakeRotator (.Roll (Math|Rotator|BreakRotator _rotator)) 0.0 (.Yaw (Math|Rotator|BreakRotator _rotator))) "1.300000,1.300000,1.300000") "Undefined" 0 0))
      (CallFunction|SearchRoomResult _returnvalue_4))
    (:6
      (bind _returnvalue_5 (Game|SpawnActorfromClass "/Game/Game/Images/Objs/Blueprint/food_BP.food_BP_C" (Math|Transform|MakeTransform _return_value (Math|Rotator|MakeRotator (.Roll (Math|Rotator|BreakRotator _rotator)) 0.0 (.Yaw (Math|Rotator|BreakRotator _rotator))) "1.300000,1.300000,1.300000") "Undefined" 0 0))
      (CallFunction|SearchRoomResult _returnvalue_5))))

(event EventBeginPlay)

(event Collision|EventActorBeginOverlap
  (params (OtherActor :type Actor%20Object%20Reference)))

(event EventTick
  (params (DeltaSeconds :type Float%20%28single-precision%29))
  (|CallParentFunction 0.0))

(fn ConstructionScript
  (|CallParentFunction))