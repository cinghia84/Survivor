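; Cellar room actor, scaled up on construction, that resolves a room search from the Value passed to its Search event.
; The first search spawns one zombie, a group of zombies or a generator at the room.
; Later searches spawn either a zombie or an item (lawn mower, bottle, stick, fuel canister) randomly ahead of the player.
; Spawned items go to SearchRoomResult, while zombie outcomes call DrawTextOnScreen.
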(event EventBeginPlay)

(event Collision|EventActorBeginOverlap
  (params (OtherActor :type Actor%20Object%20Reference)))

(event EventTick
  (params (DeltaSeconds :type Float%20%28single-precision%29)))

(event EventSearch
  (params (Value :type Integer))
  (bind _returnvalue (Math|Random|RandomFloatinRange 25.0 1e+02))
  (bind _returnvalue_2 (Math|Random|RandomFloatinRange 5e+01 1.5e+02))
  (bind _returnvalue_3 (Game|Player|GetPlayerPawn 0))
  (bind _self self)
  (bind _returnvalue_4 (Transformation|GetActorForwardVector _returnvalue_3))
  (bind _returnvalue_5 (Transformation|GetActorLocation _self))
  (bind _returnvalue_6 (Transformation|GetActorLocation _returnvalue_3))
  (bind _returnvalue_7 (* _returnvalue_4 _returnvalue))
  (bind (_x _y) (Math|Vector|BreakVector _returnvalue_5))
  (bind _returnvalue_8 (+ _returnvalue_6 _returnvalue_7))
  (bind _returnvalue_9 (+ _x _returnvalue_2))
  (bind _returnvalue_10 (+ _y _returnvalue_2))
  (bind (_x_2 _y_2) (Math|Vector|BreakVector _returnvalue_8))
  (bind _returnvalue_11 (Math|Vector|MakeVector _returnvalue_9 _returnvalue_10 118.0))
  (bind _returnvalue_12 (Math|Vector|MakeVector _x_2 _y_2 104.0))
  (bind _returnvalue_13 (Math|Conversions|ToTransform(Vector) _returnvalue_11))
  (bind _returnvalue_14 (Math|Transform|MakeTransform _returnvalue_12 "0.000000,90.000000,-90.000000" "1.300000,1.300000,1.300000"))
  (if (Variables|Default|GetFirstAccess)
    (Variables|Default|SetFirstAccess false)
    (switch int Value
      (:1
        (CallFunction|DrawTextonScreen "NewEnumerator0" :!label _label)
        (Game|SpawnActorfromClass "/Game/Characters/Zombie/Zombie_BP.Zombie_BP_C" _returnvalue_13 "AdjustIfPossibleButAlwaysSpawn" 0 0))
      (:2
        (goto _label))
      (:3
        (CallFunction|DrawTextonScreen "NewEnumerator0" :!label _label_2)
        (for _index (range 0 2)
          (Game|SpawnActorfromClass "/Game/Characters/Zombie/Zombie_BP.Zombie_BP_C" _returnvalue_13 "AdjustIfPossibleButAlwaysSpawn" 0 0)))
      (:4
        (goto _label_2))
      (:5
        (Game|SpawnActorfromClass "/Game/Game/Images/Objs/Blueprint/Generator_BP.Generator_BP_C" (Math|Transform|MakeTransform (Math|Vector|MakeVector _x _y 102.5) "0,90.000000,-90.000000" "1.000000,1.000000,1") "AdjustIfPossibleButAlwaysSpawn" 0 0 :!label _label_3))
      (:6
        (goto _label_3)))
    (else
      (switch int Value
        (:Default
          (bind _returnvalue_15 (Game|SpawnActorfromClass "/Game/Game/Images/Objs/Blueprint/lawn_mower_BP.lawn_mower_BP_C" _returnvalue_14 "Undefined" 0 0))
          (CallFunction|SearchRoomResult _returnvalue_15))
        (:1
          (Game|SpawnActorfromClass "/Game/Characters/Zombie/Zombie_BP.Zombie_BP_C" _returnvalue_13 "AdjustIfPossibleButAlwaysSpawn" 0 0)
          (CallFunction|DrawTextonScreen "NewEnumerator0"))
        (:2
          (bind _returnvalue_16 (Game|SpawnActorfromClass "/Game/Game/Images/Objs/Blueprint/bottle_BP.bottle_BP_C" _returnvalue_14 "Undefined" 0 0))
          (CallFunction|SearchRoomResult _returnvalue_16))
        (:3
          (bind _returnvalue_17 (Game|SpawnActorfromClass "/Game/Game/Images/Objs/Blueprint/stick_BP.stick_BP_C" _returnvalue_14 "Undefined" 0 0 :!label _label_4))
          (CallFunction|SearchRoomResult _returnvalue_17))
        (:4
          (goto _label_4))
        (:5
          (bind _returnvalue_18 (Game|SpawnActorfromClass "/Game/Game/Images/Objs/Blueprint/fuel_canister_BP.fuel_canister_BP_C" _returnvalue_14 "Undefined" 0 0))
          (CallFunction|SearchRoomResult _returnvalue_18))))))

(fn ConstructionScript
  (Transformation|SetActorScale3D "3.000000,3.000000,3.000000"))