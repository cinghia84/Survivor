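; Garage room actor, a searchable room that may contain a parked vehicle, items or zombies.
; On BeginPlay it destroys invisible wall, window and door components, then randomly spawns a Mini, a rusty van or nothing on the ground.
; Search maps its value to a zombie near the room or an item ahead of the player, reported through SearchRoomResult.
; SetRoofVisibility hides or shows the roof using RoofVisibility.
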(event EventBeginPlay
  (bind _self self)
  (bind _returnvalue (Transformation|GetActorLocation _self))
  (bind (_x _y) (Math|Vector|BreakVector _returnvalue))
  (Utilities|FlowControl|Sequence
    (:then_0
      (for _array_element (Utilities|Array|MakeArray (Variables|Default|GetWall4) (Variables|Default|GetWindow) (Variables|Default|GetWall7) (Variables|Default|GetWall1) (Variables|Default|GetWall6) (Variables|Default|GetWall5) (Variables|Default|GetWall3) (Variables|Default|GetWall2) (Variables|Default|GetWallDoor) (Variables|Default|GetDoorGarage1) (Variables|Default|GetDoorGarage2) (Variables|Default|GetDoorGarage3))
        (if (not (Variables|/Script/Engine.SceneComponent|GetbVisible _array_element))
          (Components|DestroyComponent _array_element))))
    (:then_1
      (bind _return_value (CallFunction|HitGroundLocation (Math|Vector|MakeVector _x _y 103.0) 2.0 (Utilities|Array|MakeArray 0)))
      (switch int (Math|Random|RandomIntegerinRange 0 6)
        (:3
          (Game|SpawnActorfromClass "/Game/Game/Images/Cars/Blueprint/Mini_BP.Mini_BP_C" (Math|Transform|MakeTransform _return_value (Math|Rotator|MakeRotator -9e+01 0.0 (.Yaw (Math|Rotator|BreakRotator (Transformation|GetActorRotation _self))))) "AdjustIfPossibleButAlwaysSpawn" 0 0 :!label _label))
        (:4
          (goto _label))
        (:5
          (Game|SpawnActorfromClass "/Game/Game/Images/Cars/Blueprint/Rusty_Van_BP.Rusty_Van_BP_C" (Math|Transform|MakeTransform _return_value (Math|Rotator|MakeRotator -9e+01 0.0 (.Yaw (Math|Rotator|BreakRotator (Transformation|GetActorRotation _self))))) "AdjustIfPossibleButAlwaysSpawn" 0 0 :!label _label_2))
        (:6
          (goto _label_2))))))

(event Collision|EventActorBeginOverlap
  (params (OtherActor :type Actor%20Object%20Reference)))

(event EventSetRoofVisibility
  (bind _returnvalue (CallFunction|RoofVisibility self))
  (Development|SetHiddeninGame (Variables|Default|GetRoof) _returnvalue true))

(event EventSearch
  (params (Value :type Integer))
  (bind _returnvalue (Math|Random|RandomFloatinRange 5e+01 1.5e+02))
  (bind _returnvalue_2 (Game|Player|GetPlayerPawn 0))
  (bind _array (Utilities|Array|MakeArray 0))
  (bind _self self)
  (bind _returnvalue_3 (Transformation|GetActorLocation _self))
  (bind (_x _y) (Math|Vector|BreakVector _returnvalue_3))
  (bind _return_value (CallFunction|HitGroundLocation (Math|Vector|MakeVector (+ _x _returnvalue) (+ _y _returnvalue) 118.0) 2e+02 _array))
  (bind (_return_value_2 _hit _rotator) (CallFunction|HitGroundLocation (+ (Transformation|GetActorLocation _returnvalue_2) (* (Transformation|GetActorForwardVector _returnvalue_2) (Math|Random|RandomFloatinRange 5e+01 1.5e+02))) 2.0 _array))
  (switch int Value
    (:Default
      (bind _returnvalue_4 (Game|SpawnActorfromClass "/Game/Game/Images/Objs/Blueprint/lawn_mower_BP.lawn_mower_BP_C" (Math|Transform|MakeTransform _return_value_2 (Math|Rotator|MakeRotator (.Roll (Math|Rotator|BreakRotator _rotator)) 0.0 (.Yaw (Math|Rotator|BreakRotator _rotator))) "1.000000,1.000000,1.000000") "Undefined" 0 0))
      (CallFunction|SearchRoomResult _returnvalue_4))
    (:1
      (Game|SpawnActorfromClass "/Game/Characters/Zombie/Zombie_BP.Zombie_BP_C" (Math|Conversions|ToTransform(Vector) _return_value) "AdjustIfPossibleButAlwaysSpawn" 0 0 :!label _label)
      (CallFunction|DrawTextonScreen "NewEnumerator0"))
    (:2
      (goto _label))
    (:3
      (goto _label))
    (:4
      (bind _returnvalue_5 (Game|SpawnActorfromClass "/Game/Game/Images/Objs/Blueprint/nail_gun_BP.nail_gun_BP_C" (Math|Transform|MakeTransform _return_value_2 (Math|Rotator|MakeRotator (.Roll (Math|Rotator|BreakRotator _rotator)) 0.0 (.Yaw (Math|Rotator|BreakRotator _rotator))) "1.000000,1.000000,1.000000") "Undefined" 0 0))
      (CallFunction|SearchRoomResult _returnvalue_5))
    (:5
      (bind _returnvalue_6 (Game|SpawnActorfromClass "/Game/Game/Images/Objs/Blueprint/garden_BP.garden_BP_C" (Math|Transform|MakeTransform _return_value_2 (Math|Rotator|MakeRotator (.Roll (Math|Rotator|BreakRotator _rotator)) 0.0 (.Yaw (Math|Rotator|BreakRotator _rotator))) "1.000000,1.000000,1.000000") "Undefined" 0 0))
      (CallFunction|SearchRoomResult _returnvalue_6))
    (:6
      (bind _returnvalue_7 (Game|SpawnActorfromClass "/Game/Game/Images/Objs/Blueprint/ladder_BP.ladder_BP_C" (Math|Transform|MakeTransform _return_value_2 (Math|Rotator|MakeRotator (.Roll (Math|Rotator|BreakRotator _rotator)) 0.0 (.Yaw (Math|Rotator|BreakRotator _rotator))) "1.000000,1.000000,1.000000") "Undefined" 0 0))
      (CallFunction|SearchRoomResult _returnvalue_7))))

(fn ConstructionScript
  (|CallParentFunction))