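; Shed room actor that can be searched for events and tool items, with a roof that can be hidden.
; BeginPlay destroys invisible wall, window and door components, and SetRoofVisibility applies the RoofVisibility result to the roof.
; The first Search uses its Value to spawn a generator, show a screen message, or show one and spawn two zombies nearby.
; Later searches spawn a tool on the ground ahead of the player and pass it to SearchRoomResult.
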(event EventBeginPlay
  (for _array_element (Utilities|Array|MakeArray (Variables|Default|GetWall5) (Variables|Default|GetWindow) (Variables|Default|GetWall8) (Variables|Default|GetWall1) (Variables|Default|GetWall6) (Variables|Default|GetWall3) (Variables|Default|GetWall4) (Variables|Default|GetWall2) (Variables|Default|GetWallDoor) (Variables|Default|GetWall7))
    (if (not (Variables|/Script/Engine.SceneComponent|GetbVisible _array_element))
      (Components|DestroyComponent _array_element))))

(event Collision|EventActorBeginOverlap
  (params (OtherActor :type Actor%20Object%20Reference)))

(event EventTick
  (params (DeltaSeconds :type Float%20%28single-precision%29))
  (|CallParentFunction 0.0))

(event EventSearch
  (params (Value :type Integer))
  (bind _returnvalue (Math|Random|RandomFloatinRange 1e+02 1.5e+02))
  (bind _returnvalue_2 (Game|Player|GetPlayerPawn 0))
  (bind _self self)
  (bind _returnvalue_3 (Transformation|GetActorLocation _self))
  (bind (_x _y) (Math|Vector|BreakVector _returnvalue_3))
  (if (Variables|Default|GetFirstAccess)
    (Variables|Default|SetFirstAccess false)
    (switch int Value
      (:1
        (Game|SpawnActorfromClass "/Game/Game/Images/Objs/Blueprint/Generator_BP.Generator_BP_C" (Math|Transform|MakeTransform (Math|Vector|MakeVector _x _y 102.5) "0,90.000000,-90.000000" "1.300000,1.300000,1.300000") "AdjustIfPossibleButAlwaysSpawn" 0 0 :!label _label))
      (:2
        (goto _label))
      (:3
        (CallFunction|DrawTextonScreen "NewEnumerator1" :!label _label_2))
      (:4
        (goto _label_2))
      (:5
        (CallFunction|DrawTextonScreen "NewEnumerator0" :!label _label_3)
        (for _index (range 0 1)
          (Game|SpawnActorfromClass "/Game/Characters/Zombie/Zombie_BP.Zombie_BP_C" (Math|Conversions|ToTransform(Vector) (Math|Vector|MakeVector (+ _x _returnvalue) (+ _y _returnvalue) 118.0)) "AdjustIfPossibleButAlwaysSpawn" 0 0)))
      (:6
        (goto _label_3)))
    (else
      (bind (_return_value _hit _rotator) (CallFunction|HitGroundLocation (+ (Transformation|GetActorLocation _returnvalue_2) (* (Transformation|GetActorForwardVector _returnvalue_2) (Math|Random|RandomFloatinRange 5e+01 1.5e+02))) 2.0 (Utilities|Array|MakeArray 0)))
      (switch int Value
        (:Default
          (bind _returnvalue_4 (Game|SpawnActorfromClass "/Game/Game/Images/Objs/Blueprint/chainsaw_BP.chainsaw_BP_C" (Math|Transform|MakeTransform _return_value (Math|Rotator|MakeRotator (.Roll (Math|Rotator|BreakRotator _rotator)) 0.0 (.Yaw (Math|Rotator|BreakRotator _rotator))) "1.000000,1.000000,1.000000") "Undefined" 0 0))
          (CallFunction|SearchRoomResult _returnvalue_4))
        (:1
          (bind _returnvalue_5 (Game|SpawnActorfromClass "/Game/Game/Images/Objs/Blueprint/ladder_BP.ladder_BP_C" (Math|Transform|MakeTransform _return_value (Math|Rotator|MakeRotator (.Roll (Math|Rotator|BreakRotator _rotator)) 0.0 (.Yaw (Math|Rotator|BreakRotator _rotator))) "1.000000,1.000000,1.000000") "Undefined" 0 0))
          (CallFunction|SearchRoomResult _returnvalue_5))
        (:2
          (bind _returnvalue_6 (Game|SpawnActorfromClass "/Game/Game/Images/Objs/Blueprint/hammer_BP.hammer_BP_C" (Math|Transform|MakeTransform _return_value (Math|Rotator|MakeRotator (.Roll (Math|Rotator|BreakRotator _rotator)) 0.0 (.Yaw (Math|Rotator|BreakRotator _rotator))) "1.000000,1.000000,1.000000") "Undefined" 0 0))
          (CallFunction|SearchRoomResult _returnvalue_6))
        (:3
          (bind _returnvalue_7 (Game|SpawnActorfromClass "/Game/Game/Images/Objs/Blueprint/torch_BP.torch_BP_C" (Math|Transform|MakeTransform _return_value (Math|Rotator|MakeRotator (.Roll (Math|Rotator|BreakRotator _rotator)) 0.0 (.Yaw (Math|Rotator|BreakRotator _rotator))) "1.000000,1.000000,1.000000") "Undefined" 0 0))
          (CallFunction|SearchRoomResult _returnvalue_7))
        (:4
          (bind _returnvalue_8 (Game|SpawnActorfromClass "/Game/Game/Images/Objs/Blueprint/power_tools_BP.power_tools_BP_C" (Math|Transform|MakeTransform _return_value (Math|Rotator|MakeRotator (.Roll (Math|Rotator|BreakRotator _rotator)) 0.0 (.Yaw (Math|Rotator|BreakRotator _rotator))) "1.000000,1.000000,1.000000") "Undefined" 0 0))
          (CallFunction|SearchRoomResult _returnvalue_8))
        (:5
          (bind _returnvalue_9 (Game|SpawnActorfromClass "/Game/Game/Images/Objs/Blueprint/lawn_mower_BP.lawn_mower_BP_C" (Math|Transform|MakeTransform _return_value (Math|Rotator|MakeRotator (.Roll (Math|Rotator|BreakRotator _rotator)) 0.0 (.Yaw (Math|Rotator|BreakRotator _rotator))) "1.000000,1.000000,1.000000") "Undefined" 0 0))
          (CallFunction|SearchRoomResult _returnvalue_9))))))

(event EventSetRoofVisibility
  (bind _returnvalue (CallFunction|RoofVisibility self))
  (Development|SetHiddeninGame (Variables|Default|GetRoof) _returnvalue true))

(fn ConstructionScript
  (|CallParentFunction))