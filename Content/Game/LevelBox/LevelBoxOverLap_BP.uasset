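; LevelBoxOverLap_BP is a trigger box that streams in a level when the TopDownCharacter enters it.
; Begin overlap creates an instance of LevelNameLoad, shows it and records its world asset in DoNGameInstance's LoadedLevelArray, or prints if already recorded.
; The instance name always resolves to "TEST0" because the random range is zero.
; End overlap checks LevelNameUnload but instances LevelNameLoad and sets ShouldBeLoaded true, so it never unloads anything.
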(event OnComponentBeginOverlap(Box)
  (params (OverlappedComponent :type Primitive%20Component%20Object%20Reference) (OtherActor :type Actor%20Object%20Reference) (OtherComp :type Primitive%20Component%20Object%20Reference) (OtherBodyIndex :type Integer) (bFromSweep :type Boolean) (SweepResult :type Hit%20Result%20Structure%20%28by%20ref%29))
  (if (Utilities|Name|NotEqual(Name) (Variables|Default|GetLevelNameLoad) "None")
    (Utilities|Casting|CastToTopDownCharacter OtherActor)
    (bind _asdo_ngame_instance (Utilities|Casting|CastToDoNGameInstance (Game|GetGameInstance)))
    (bind _output_get (Variables|Default|SetLevelInstanceName (Utilities|String|Append "TEST" (Utilities|String|ToString(Integer) (Math|Random|RandomInteger 0)))))
    (bind _returnvalue (Class|LevelStreaming|CreateInstance (Class|GameplayStatics|GetStreamingLevel (Variables|Default|GetLevelNameLoad)) _output_get))
    (if (== (Utilities|Array|FindItem (Variables|/Game/TopDownBP/Blueprints/DoNGameInstance.DoNGameInstance_C|GetLoadedLevelArray _asdo_ngame_instance) (Variables|/Script/Engine.LevelStreaming|GetWorldAsset _returnvalue)) -1)
      (Variables|/Script/Engine.LevelStreaming|SetbShouldBeLoaded _returnvalue true)
      (Variables|/Script/Engine.LevelStreaming|SetbShouldBeVisible _returnvalue true)
      (Variables|Default|SetLoaded true)
      (bind _asdo_ngame_instance_2 (Utilities|Casting|CastToDoNGameInstance (Game|GetGameInstance)))
      (Utilities|Array|Add (Variables|/Game/TopDownBP/Blueprints/DoNGameInstance.DoNGameInstance_C|GetLoadedLevelArray _asdo_ngame_instance_2) (Variables|/Script/Engine.LevelStreaming|GetWorldAsset _returnvalue))
      (else
        (Development|PrintString "Hello" true false "(R=0.000000,G=0.660000,B=1.000000,A=1.000000)" 5.0)))))

(event OnComponentEndOverlap(Box)
  (params (OverlappedComponent :type Primitive%20Component%20Object%20Reference) (OtherActor :type Actor%20Object%20Reference) (OtherComp :type Primitive%20Component%20Object%20Reference) (OtherBodyIndex :type Integer))
  (if (Utilities|Name|NotEqual(Name) (Variables|Default|GetLevelNameUnload) "None")
    (Utilities|Casting|CastToTopDownCharacter OtherActor)
    (bind _returnvalue (Class|LevelStreaming|CreateInstance (Class|GameplayStatics|GetStreamingLevel (Variables|Default|GetLevelNameLoad)) (Variables|Default|GetLevelInstanceName)))
    (if (Class|LevelStreaming|IsLevelLoaded _returnvalue)
      (Variables|/Script/Engine.LevelStreaming|SetbShouldBeLoaded _returnvalue true))))

(event EventBeginPlay)

(event Collision|EventActorBeginOverlap
  (params (OtherActor :type Actor%20Object%20Reference)))

(event EventTick
  (params (DeltaSeconds :type Float%20%28single-precision%29)))

(fn ConstructionScript)